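; Base RPG player controller handling input mappings, targeting, tooltips and travel transitions, with stub functions apparently meant for child overrides.
; Initialization caches the RPGSystem, sets up the HUD and fades in; disable-input crowd control clears mappings and UI.
; Mouse line traces with sphere-trace fallbacks find interactables, while separate selectors maintain highlighted, selected and skill-target states.
; Client events handle server-travel countdowns, with a timed fade failback.
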(event `EnhancedInput|/Game/RPGSystem/Examples/TopDown/Input/Actions/IA_TakeItemAround`
  (params (ActionValue :type Boolean) (ElapsedSeconds :type "Float (double-precision)") (TriggeredSeconds :type "Float (double-precision)") (InputAction :type "InputAction Object Reference" :default "/Game/RPGSystem/Examples/TopDown/Input/Actions/IA_TakeItemAround.IA_TakeItemAround"))
  (bind _rpgsystem (`self.RPGSystem`))
  ;[1 1 1] Take all Items
  (:`Started`
    (`/Engine/EditorBlueprintResources/StandardMacros.IsValid` _rpgsystem
      (:`Is Valid`
        (`/Game/RPGSystem/Blueprints/BPC_RPGSystem.TakeAllItemsServer` _rpgsystem (`/Game/RPGSystem/Blueprints/BPC_RPGSystem.PickupMinGrade` _rpgsystem))))))

(event `self.ReceiveBeginPlay`
  (bind ((`MoveToTrace_21_08C3CD004AA60B33DC00BCB3DC60857C` _movetotrace) (`InteractTraceType_27_34121EF24AA1D8233FF7B283306CA093` _interacttracetype)) (break `/Game/RPGSystem/Blueprints/Structure/Settings/S_Settings_Traces` (`.TraceObjectTypes_124_C5F9E9754912A336B98600A0E0E8BCEE` (break `/Game/RPGSystem/Blueprints/Structure/Settings/S_Settings` (`/Game/RPGSystem/Blueprints/Utilities/BPL_RPG_Utilities.GetGlobalSettings`)))))
  ;[1 1 1] Comment
  (set `self.InteractTrace` _interacttracetype)
  (set `self.Move to Trace` _movetotrace)
  (if (`self.IsLocalPlayerController`)
    (message `/Game/RPGSystem/Blueprints/Utilities/BPI_RPG_PlayerCamera.SetManualCameraFadeWithHUD` (`GameplayStatics.GetPlayerCameraManager` 0) 1.0 (struct :`A` 1.0) false)))

(event `EnhancedInput|/Game/RPGSystem/Examples/TopDown/Input/Actions/IA_ShowItemTooltip`
  (params (ActionValue :type Boolean) (ElapsedSeconds :type "Float (double-precision)") (TriggeredSeconds :type "Float (double-precision)") (InputAction :type "InputAction Object Reference" :default "/Game/RPGSystem/Examples/TopDown/Input/Actions/IA_ShowItemTooltip.IA_ShowItemTooltip"))
  (bind _returnvalue (`self.GetHUD`))
  ;[1 1 1] Show tooltip
  (:`Started`
    (message `/Game/RPGSystem/Blueprints/Utilities/BPI_RPG_HUD.ToggleWorldTooltip` _returnvalue true))
  (:`Canceled`
    (message `/Game/RPGSystem/Blueprints/Utilities/BPI_RPG_HUD.ToggleWorldTooltip` _returnvalue false :!label _label))
  (:`Completed`
    (goto _label)))

(event `/Game/RPGSystem/Blueprints/Utilities/BPI_RPG_PlayerController.OnRPG_CharacterInitialized`
  (params (RPGSystem :type "/Game/RPGSystem/Blueprints/BPC_RPGSystem Object Reference"))
  ;[1 1 1] Comment
  (bind _output_get (set `self.RPGSystem` RPGSystem))
  (add `/Game/RPGSystem/Blueprints/BPC_RPGSystem.OnCrowdControlChanged` _output_get (`|CreateDelegate` :!event `OnCrowdControlChanged`))
  (if (`self.IsLocalPlayerController`)
    (message `/Game/RPGSystem/Blueprints/Utilities/BPI_RPG_HUD.InitHUD` (`/Game/RPGSystem/Blueprints/Utilities/BPL_RPG_Utilities.GetHUD`) (`self.RPGSystem`))
    (message `/Game/RPGSystem/Blueprints/Utilities/BPI_RPG_PlayerCamera.StartCameraFadeWithHUD` (`GameplayStatics.GetPlayerCameraManager` 0) 1.0 0.0 1.0 (struct :`A` 1.0) true true)
    (`KismetSystemLibrary.Delay` 0.5)
    (if (`self.IsLocalController`)
      (`self.GiveInputMapping`))))

(event `self.ReceiveUnPossess`
  (params (UnpossessedPawn :type "Pawn Object Reference"))
  (bind _returnvalue (subsystem `EnhancedInputLocalPlayerSubsystem`))
  ;[1 1 1] Remove Input Mapping if Pawn got destroyed
  (if (`self.IsLocalPlayerController`)
    (`/Engine/EditorBlueprintResources/StandardMacros.IsValid` _returnvalue
      (:`Is Valid`
        (`EnhancedInputSubsystemInterface.ClearAllMappings` _returnvalue) ; Need to be replicated sind UnPossess only gets called on the Server (iirc)
      )
      (:`Is Not Valid`
        _)))
  (set `self.RPGSystem` null)
  (`parent.ReceiveUnPossess` UnpossessedPawn))

(event `Client_ServerTravelInitialized`
  (params (TravelTime :type "Float (double-precision)") (Waypoint :type Name))
  (bind _returnvalue (- TravelTime (`GameStateBase.GetServerWorldTimeSeconds` (`GameplayStatics.GetGameState`))))
  ;[1 1 1] Server Travel
  (if (> _returnvalue 0.0)
    (bind _returnvalue_2 (`KismetSystemLibrary.K2_SetTimerDelegate` (`|CreateDelegate` :!event `OnTravelStarted`) _returnvalue))
    (set `self.TravelTimer` _returnvalue_2)
    (if (> _returnvalue 1.0)
      (message `/Game/RPGSystem/Blueprints/Utilities/BPI_RPG_HUD.DisplayTravelCountdown` (`self.GetHUD`) TravelTime Waypoint))))

(event `OnSeamlessTravelFinished`
  (params (RPGSystem :type "/Game/RPGSystem/Blueprints/BPC_RPGSystem Object Reference"))
  (`self.OnRPG_CharacterInitialized` RPGSystem))

(event `/Game/RPGSystem/Blueprints/Utilities/BPI_RPG_PlayerController.ServerTravel_Initialized`
  (params (TravelTime :type "Float (double-precision)") (Waypoint :type Name))
  ;[1 1 1] Server Travel
  (`self.Client_ServerTravelInitialized` TravelTime Waypoint))

(event `/Game/RPGSystem/Blueprints/Utilities/BPI_RPG_PlayerController.ServerTravel_Canceled`
  ;[1 1 1] Server Travel
  (`self.Client_ServerTravelCaneled`))

(event `Client_ServerTravelCaneled`
  ;[1 1 1] Server Travel
  (`KismetSystemLibrary.K2_ClearAndInvalidateTimerHandle` (`self.TravelTimer`))
  (`PlayerCameraManager.StopCameraFade` (`GameplayStatics.GetPlayerCameraManager` 0))
  (message `/Game/RPGSystem/Blueprints/Utilities/BPI_RPG_HUD.RemoveTravelCountdown` (`self.GetHUD`)))

(event `OnTravelStarted`
  ;[1 1 1] Server Travel
  (message `/Game/RPGSystem/Blueprints/Utilities/BPI_RPG_PlayerCamera.StartCameraFadeWithHUD` (`GameplayStatics.GetPlayerCameraManager` 0) 0.0 1.0 1.0 (struct :`A` 1.0) true true)
  (`KismetSystemLibrary.Delay` 15.0) ; Failback incase something went wrong, wont get triggered if travel succeed
  (message `/Game/RPGSystem/Blueprints/Utilities/BPI_RPG_PlayerCamera.StopCameraFadeWithHUD` (`GameplayStatics.GetPlayerCameraManager` 0)))

(fn `GetInteractableUnderMouse`
  (returns (Success :type Boolean) (Target :type "Actor Object Reference") (Action :type "/Game/RPGSystem/Blueprints/Enum/Interact/E_InteractAction Enum"))
  (locals (Hit :type "HitResult Structure") (VarAction :type "/Game/RPGSystem/Blueprints/Enum/Interact/E_InteractAction Enum" :default "NewEnumerator0") (VarTarget :type "Actor Object Reference") (VarTargetComp :type "PrimitiveComponent Object Reference") (VarStart :type "Vector Structure" :default (0.0 0.0 0.0)) (VarMouseDir :type "Vector Structure" :default (0.0 0.0 0.0)) (VarEnd :type "Vector Structure" :default (0.0 0.0 0.0)))
  (bind (_worldlocation _worlddirection) (`self.DeprojectMousePositionToWorld`))
  (bind _varend (`local.VarEnd`))
  (bind (_bblockinghit _binitialoverlap _time _distance _location _impactpoint _normal _impactnormal _physmat _hitactor _hitcomponent _hitbonename _bonename _hititem _elementindex _faceindex _tracestart _traceend) (`GameplayStatics.BreakHitResult` (`local.Hit`)))
  (set `local.VarStart` _worldlocation)
  (set `local.VarMouseDir` _worlddirection)
  (bind _outhit (`KismetSystemLibrary.LineTraceSingle` _worldlocation (+ _worldlocation (* (`local.VarMouseDir`) 3000.0)) (`self.InteractTrace`) false (`|MakeArray` (`self.K2_GetPawn`) :!type "Actor Object Reference")))
  (bind _output_get (set `local.Hit` _outhit))
  (bind (_bblockinghit_2 _binitialoverlap_2 _time_2 _distance_2 _location_2 _impactpoint_2 _normal_2 _impactnormal_2 _physmat_2 _hitactor_2) (`GameplayStatics.BreakHitResult` _output_get))
  (bind (_success _type _action) (message `/Game/RPGSystem/Blueprints/Utilities/BPI_RPG_Interaction.GetInteractInfo` _hitactor_2 (`self.RPGSystem`)))
  (if _success
    (set `local.VarTarget` _hitactor_2)
    (set `local.VarAction` _action)
    (return true (`local.VarTarget`) (`local.VarAction`))
    (else
      (set `local.VarEnd` (`KismetMathLibrary.SelectVector` _impactpoint _traceend (or _bblockinghit _binitialoverlap)))
      (bind _outhits (`KismetSystemLibrary.SphereTraceMulti` (`local.VarStart`) (`local.VarEnd`) (`self.InteractTraceRadius`) (`self.InteractTrace`) false (`|MakeArray` (`self.K2_GetPawn`) (`ActorComponent.GetOwner` (`self.RPGSystem`)) :!type "Actor Object Reference")))
      (bind (_success_2 _nearestactor _nearestcomp _distance_3 _action_2) (`/Game/RPGSystem/Blueprints/Utilities/BPL_RPG_Utilities.GetNearestInteractableActorOutHits` (`self.RPGSystem`) (`local.VarEnd`) _outhits))
      (if _success_2
        (set `local.VarTarget` _nearestactor)
        (set `local.VarAction` _action_2)
        (return true (`local.VarTarget`) (`local.VarAction`))
        (else
          (bind _outhits_2 (`KismetSystemLibrary.SphereTraceMulti` _varend _varend (`self.InteractTraceRadius`) (`self.InteractTrace`)))
          (bind (_success_3 _nearestactor_2 _nearestcomp_2 _distance_4 _action_3) (`/Game/RPGSystem/Blueprints/Utilities/BPL_RPG_Utilities.GetNearestInteractableActorOutHits` (`self.RPGSystem`) _varend _outhits_2))
          (if _success_3
            (set `local.VarTarget` _nearestactor_2)
            (set `local.VarAction` _action_3)
            (return true (`local.VarTarget`) (`local.VarAction`))
            (else
              (return false null "NewEnumerator0"))))))))

(fn `GetInteractionRange`
  (returns (Range :type "Float (double-precision)"))
  (return 0.0))

(fn `GetMoveToMouseLocation`
  (returns (bBlockingHit :type Boolean) (Location :type "Vector Structure") (HitActor :type "Actor Object Reference") (HitComponent :type "PrimitiveComponent Object Reference"))
  (bind (_worldlocation _worlddirection) (`self.DeprojectMousePositionToWorld`))
  (bind _outhit (`KismetSystemLibrary.LineTraceSingle` _worldlocation (+ _worldlocation (* _worlddirection 3000.0)) (`self.Move to Trace`) false (`|MakeArray` (`self.K2_GetPawn`) (`ActorComponent.GetOwner` (`self.RPGSystem`)) :!type "Actor Object Reference")))
  (bind (_bblockinghit _binitialoverlap _time _distance _location _impactpoint _normal _impactnormal _physmat _hitactor _hitcomponent _hitbonename _bonename _hititem _elementindex _faceindex _tracestart _traceend) (`GameplayStatics.BreakHitResult` _outhit))
  (return _bblockinghit (`KismetMathLibrary.SelectVector` _location _traceend _bblockinghit) _hitactor _hitcomponent))

(fn `GiveInputMapping`
  (if (`self.IsLocalPlayerController`)
    _))

(fn `IsGamepad`
  (returns (Return :type Boolean))
  (return false))

(fn `IsLocal`
  (returns (ReturnValue :type Boolean))
  (return (`self.IsLocalPlayerController`)))

(fn `OnCrowdControlChanged`
  (params (Type :type "/Game/RPGSystem/Blueprints/Enum/Basic/E_CrowdControlType Enum" :default "NewEnumerator0") (State :type "/Game/RPGSystem/Blueprints/Enum/Basic/E_SE_CC_State Enum" :default "NewEnumerator0"))
  (switch `/Game/RPGSystem/Blueprints/Enum/Basic/E_CrowdControlType` Type
    (:`NewEnumerator10`
      (switch `/Game/RPGSystem/Blueprints/Enum/Basic/E_SE_CC_State` State
        (:`NewEnumerator0`
          (`self.RemoveInputMapping`))
        (:`NewEnumerator2`
          (`self.GiveInputMapping`))))))

(fn `ReleaseHotbar`
  (params (Index :type Integer))
  (bind _return (`/Game/RPGSystem/Blueprints/BPC_RPGSystem.GetHotbar` (`self.RPGSystem`) Index))
  (bind ((`ID_12_F30D2A154C3F52D425D9D2AE8986FD0C` _id) (`IsSkill_14_276FB76F476651A7E742D4994C69E5E2` _isskill)) (break `/Game/RPGSystem/Blueprints/Structure/SaveGame/S_HotbarEntry` _return))
  (if _isskill
    (`/Game/RPGSystem/Blueprints/BPC_RPGSystem.ReleaseSkillServer` (`self.RPGSystem`) _id)))

(fn `RemoveInputMapping`
  (bind _returnvalue (`self.GetHUD`))
  (if (`self.IsLocalPlayerController`)
    (`EnhancedInputSubsystemInterface.ClearAllMappings` (subsystem `EnhancedInputLocalPlayerSubsystem`))
    (message `/Game/RPGSystem/Blueprints/Utilities/BPI_RPG_PlayerCharacter.StopMovementInterface` (`self.K2_GetPawn`))
    (bind _list (message `/Game/RPGSystem/Blueprints/Utilities/BPI_RPG_HUD.GetOpenUI_List` _returnvalue))
    (`/Game/RPGSystem/Blueprints/Utilities/BML_RPG_Utilities.ForeachLoopByRef` _list
      (:`Body`
        (message `/Game/RPGSystem/Blueprints/Utilities/BPI_RPG_HUD.CloseLastOpenUI` _returnvalue)))))

(fn `SelectInteractable`
  (params (Target :type "Actor Object Reference"))
  (bind _returnvalue (`self.GetHUD`))
  (bind _rpgsystem (`self.RPGSystem`))
  (bind _selectedinteractable (`/Game/RPGSystem/Blueprints/BPC_RPGSystem.SelectedInteractable` _rpgsystem))
  (bind _selectedinteractable_2 (`/Game/RPGSystem/Blueprints/BPC_RPGSystem.SelectedInteractable` (`self.RPGSystem`)))
  (bind _selectedinteractable_3 (`/Game/RPGSystem/Blueprints/BPC_RPGSystem.SelectedInteractable` (`self.RPGSystem`)))
  (`/Engine/EditorBlueprintResources/StandardMacros.IsValid` Target
    (:`Is Valid`
      (if (`KismetSystemLibrary.IsValid` _selectedinteractable_3)
        (if (== _selectedinteractable_3 (`local.Target`))
          ;[1 1 1] Again current | check if its an Item and if we want to display the ItemTooltip
          (bind _asbp_item_base (cast `/Game/RPGSystem/Blueprints/Item/BP_Item_Base` (`/Game/RPGSystem/Blueprints/BPC_RPGSystem.SelectedInteractable` (`self.RPGSystem`))))
          (message `/Game/RPGSystem/Blueprints/Utilities/BPI_RPG_HUD.HandleItemTooltip` (`self.GetHUD`) _asbp_item_base (`|GetInputActionValue`))
          (else
            (if (`self.MoveToAction`)
              (set `self.MoveToAction` false))
            (`|ExecutionSequence`
              (:`then_0`
                ;[1 1 1] Unselect current
                (if (and (!= _selectedinteractable (`/Game/RPGSystem/Blueprints/BPC_RPGSystem.HighlightedInteractable` _rpgsystem)) (!= _selectedinteractable (`/Game/RPGSystem/Blueprints/BPC_RPGSystem.SelectedSkillTarget` _rpgsystem))) :!label _label
                  (message `/Game/RPGSystem/Blueprints/Utilities/BPI_RPG_Interaction.SelectInteractable` _selectedinteractable_2 false)
                  (message `/Game/RPGSystem/Blueprints/Utilities/BPI_RPG_HUD.SetWorldTooltipVisibility` (`self.GetHUD`) _selectedinteractable_2 false))
                (message `/Game/RPGSystem/Blueprints/Utilities/BPI_RPG_HUD.HandleScreenTooltip` _returnvalue null null false)
                (message `/Game/RPGSystem/Blueprints/Utilities/BPI_RPG_HUD.HandleItemTooltip` _returnvalue null false)
                (set `/Game/RPGSystem/Blueprints/BPC_RPGSystem.SelectedInteractable` null (`self.RPGSystem`)))
              (:`then_1`
                ;[1 1 1] Select New
                (bind _output_get (set `/Game/RPGSystem/Blueprints/BPC_RPGSystem.SelectedInteractable` (`local.Target`) (`self.RPGSystem`) :!label _label_2))
                (message `/Game/RPGSystem/Blueprints/Utilities/BPI_RPG_Interaction.SelectInteractable` _output_get true)
                (message `/Game/RPGSystem/Blueprints/Utilities/BPI_RPG_HUD.SetWorldTooltipVisibility` (`self.GetHUD`) _output_get true)
                (if (`|GetInputActionValue`)
                  (bind _asbp_item_base_2 (cast `/Game/RPGSystem/Blueprints/Item/BP_Item_Base` (`/Game/RPGSystem/Blueprints/BPC_RPGSystem.SelectedInteractable` (`self.RPGSystem`))))
                  (message `/Game/RPGSystem/Blueprints/Utilities/BPI_RPG_HUD.HandleItemTooltip` (`self.GetHUD`) _asbp_item_base_2 true))))))
        (else
          (goto _label_2))))
    (:`Is Not Valid`
      (`/Engine/EditorBlueprintResources/StandardMacros.IsValid` (`/Game/RPGSystem/Blueprints/BPC_RPGSystem.SelectedInteractable` (`self.RPGSystem`))
        (:`Is Valid`
          (goto _label))))))

(fn `SelectObject`
  (params (Target :type "Actor Object Reference"))
  (bind _returnvalue (`self.GetHUD`))
  (bind _rpgsystem (`self.RPGSystem`))
  (bind _highlightedinteractable (`/Game/RPGSystem/Blueprints/BPC_RPGSystem.HighlightedInteractable` (`self.RPGSystem`)))
  (bind _highlightedinteractable_2 (`/Game/RPGSystem/Blueprints/BPC_RPGSystem.HighlightedInteractable` (`self.RPGSystem`)))
  (bind _highlightedinteractable_3 (`/Game/RPGSystem/Blueprints/BPC_RPGSystem.HighlightedInteractable` _rpgsystem))
  (`/Engine/EditorBlueprintResources/StandardMacros.IsValid` Target
    (:`Is Valid`
      (if (`KismetSystemLibrary.IsValid` _highlightedinteractable_2)
        (if (== _highlightedinteractable_2 (`local.Target`))
          ;[1 1 1] Again current | check if its an Item and if we want to display the ItemTooltip
          (bind _asbp_item_base (cast `/Game/RPGSystem/Blueprints/Item/BP_Item_Base` (`/Game/RPGSystem/Blueprints/BPC_RPGSystem.HighlightedInteractable` (`self.RPGSystem`))))
          (message `/Game/RPGSystem/Blueprints/Utilities/BPI_RPG_HUD.HandleItemTooltip` (`self.GetHUD`) _asbp_item_base (`|GetInputActionValue`))
          (else
            (`|ExecutionSequence`
              (:`then_0`
                ;[1 1 1] Unselect current
                (if (and (!= _highlightedinteractable_3 (`/Game/RPGSystem/Blueprints/BPC_RPGSystem.SelectedInteractable` _rpgsystem)) (!= _highlightedinteractable_3 (`/Game/RPGSystem/Blueprints/BPC_RPGSystem.SelectedSkillTarget` _rpgsystem)) (not (`|GetInputActionValue`))) :!label _label
                  (message `/Game/RPGSystem/Blueprints/Utilities/BPI_RPG_Interaction.SelectInteractable` _highlightedinteractable false)
                  (message `/Game/RPGSystem/Blueprints/Utilities/BPI_RPG_HUD.SetWorldTooltipVisibility` (`self.GetHUD`) _highlightedinteractable false))
                (message `/Game/RPGSystem/Blueprints/Utilities/BPI_RPG_HUD.HandleScreenTooltip` _returnvalue null null false)
                (message `/Game/RPGSystem/Blueprints/Utilities/BPI_RPG_HUD.HandleItemTooltip` _returnvalue null false)
                (set `/Game/RPGSystem/Blueprints/BPC_RPGSystem.HighlightedInteractable` null (`self.RPGSystem`)))
              (:`then_1`
                ;[1 1 1] Select New
                (bind _output_get (set `/Game/RPGSystem/Blueprints/BPC_RPGSystem.HighlightedInteractable` (`local.Target`) (`self.RPGSystem`) :!label _label_2))
                (message `/Game/RPGSystem/Blueprints/Utilities/BPI_RPG_Interaction.SelectInteractable` _output_get true)
                (message `/Game/RPGSystem/Blueprints/Utilities/BPI_RPG_HUD.SetWorldTooltipVisibility` (`self.GetHUD`) _output_get true)
                (if (`|GetInputActionValue`)
                  (bind _asbp_item_base_2 (cast `/Game/RPGSystem/Blueprints/Item/BP_Item_Base` (`/Game/RPGSystem/Blueprints/BPC_RPGSystem.HighlightedInteractable` (`self.RPGSystem`))))
                  (message `/Game/RPGSystem/Blueprints/Utilities/BPI_RPG_HUD.HandleItemTooltip` (`self.GetHUD`) _asbp_item_base_2 true))))))
        (else
          (goto _label_2))))
    (:`Is Not Valid`
      (`/Engine/EditorBlueprintResources/StandardMacros.IsValid` (`/Game/RPGSystem/Blueprints/BPC_RPGSystem.HighlightedInteractable` (`self.RPGSystem`))
        (:`Is Valid`
          (goto _label))))))

(fn `SelectTarget`
  (params (Target :type "Actor Object Reference"))
  (locals (VarNewTarget :type "/Game/RPGSystem/Blueprints/BPC_RPGSystem Object Reference"))
  (bind (_valid _target_) (`/Game/RPGSystem/Blueprints/Utilities/BPL_RPG_Utilities.IsValidTarget` (`self.RPGSystem`) (`local.Target`)))
  (bind _selectedskilltarget (`/Game/RPGSystem/Blueprints/BPC_RPGSystem.SelectedSkillTarget` (`self.RPGSystem`)))
  (`/Engine/EditorBlueprintResources/StandardMacros.IsValid` Target
    (:`Is Valid`
      (if _valid
        (set `local.VarNewTarget` _target_)
        ;[1 1 1] Select
        (if (`KismetSystemLibrary.IsValid` _selectedskilltarget)
          (if (not (== _selectedskilltarget (`local.VarNewTarget`)))
            (if (`self.MoveToAction`)
              (set `self.MoveToAction` false))
            (bind _output_get (set `/Game/RPGSystem/Blueprints/BPC_RPGSystem.SelectedSkillTarget` (`local.VarNewTarget`) (`self.RPGSystem`) :!label _label))
            (message `/Game/RPGSystem/Blueprints/Utilities/BPI_RPG_Interaction.SelectInteractable` (`ActorComponent.GetOwner` _output_get) true))
          (else
            (goto _label)))
        (else
          ;[1 1 1] Unselect
          (if (`KismetSystemLibrary.IsValid` (`/Game/RPGSystem/Blueprints/BPC_RPGSystem.SelectedSkillTarget` (`self.RPGSystem`))) :!label _label_2
            (message `/Game/RPGSystem/Blueprints/Utilities/BPI_RPG_Interaction.SelectInteractable` (`ActorComponent.GetOwner` (`/Game/RPGSystem/Blueprints/BPC_RPGSystem.SelectedSkillTarget` (`self.RPGSystem`))) false)
            (set `/Game/RPGSystem/Blueprints/BPC_RPGSystem.SelectedSkillTarget` null (`self.RPGSystem`))
            (else
              (set `/Game/RPGSystem/Blueprints/BPC_RPGSystem.SelectedSkillTarget` null (`self.RPGSystem`)))))))
    (:`Is Not Valid`
      (goto _label_2))))

(fn `UserConstructionScript`)