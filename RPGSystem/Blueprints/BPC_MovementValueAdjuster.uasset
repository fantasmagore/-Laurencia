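; Actor component that adjusts its owner's walk speed, switching between a supplied speed and the global default.
; It caches acceleration, braking friction and walking deceleration from the movement component, fetched by interface message, on BeginPlay or first adjustment.
; Each adjustment restores cached braking values and scales cached acceleration by a factor derived from the default walk speed, never below one, regardless of the requested speed.
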(event `self.ReceiveBeginPlay`
  (`self.Init`))

(fn `AdjustMovementParameter`
  (params (ToDefault :type Boolean) (Speed :type "Float (double-precision)"))
  (bind ((`DefaultWalkSpeed_54_629F3C4B45082534F455A4B5A9FBBCE4` _defaultwalkspeed)) (break `/Game/RPGSystem/Blueprints/Structure/Settings/S_Settings` (`/Game/RPGSystem/Blueprints/Utilities/BPL_RPG_Utilities.GetGlobalSettings`)))
  (if (not (`self.bInit`))
    (`self.Init`))
  (bind _component (message `/Game/RPGSystem/Blueprints/Utilities/BPI_RPG_PlayerCharacter.GetCharacterMovementComponent` (`self.GetOwner`)))
  (set `CharacterMovementComponent.MaxWalkSpeed` (`KismetMathLibrary.SelectFloat` _defaultwalkspeed Speed ToDefault) _component)
  (set `CharacterMovementComponent.MaxAcceleration` (* (`KismetMathLibrary.FMax` (/ 2000.0 _defaultwalkspeed) 1.0) (`self.Cached_MaxAcceleration`)) _component)
  (set `CharacterMovementComponent.BrakingFriction` (`self.Cached_BrakingFriction`) _component)
  (set `CharacterMovementComponent.BrakingDecelerationWalking` (`self.Cached_BrakingDecelerationWalking`) _component))

(fn `Init`
  (bind _component (message `/Game/RPGSystem/Blueprints/Utilities/BPI_RPG_PlayerCharacter.GetCharacterMovementComponent` (`self.GetOwner`)))
  (set `self.Cached_MaxAcceleration` (`CharacterMovementComponent.GetMaxAcceleration` _component))
  (set `self.Cached_BrakingFriction` (`CharacterMovementComponent.BrakingFriction` _component))
  (set `self.Cached_BrakingDecelerationWalking` (`CharacterMovementComponent.BrakingDecelerationWalking` _component))
  (set `self.bInit` true))