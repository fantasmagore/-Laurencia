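; Base AI character for the RPG system, used for enemies and followers, delegating stats and state to BPCRPGSystemAI and answering interaction and targeting queries.
; Component events create and update a floating health bar and handle death.
; Tick sets movement-based rotation and stops crowd-controlled movement.
; On death it ragdolls, swaps the settled mesh for a frozen poseable copy, then destroys itself once unseen or past a time limit.
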(event `OnResourceTypeChanged`
  (params (Type :type "/Game/RPGSystem/Blueprints/Enum/Basic/E_ResourceType Enum" :default "NewEnumerator0") (Last :type "Float (double-precision)") (FromSE :type Boolean))
  (bind _bpc_rpgsystem_ai (`self.BPC_RPGSystem_AI`))
  (bind _mesh (`self.Mesh`))
  (bind _bpc_rpgsystem_ai_2 (`self.BPC_RPGSystem_AI`))
  ;[1 1 1] HealthBar Widget / HIt sound
  (switch `/Game/RPGSystem/Blueprints/Enum/Basic/E_ResourceType` Type
    (:`NewEnumerator0`
      (if (`/Game/RPGSystem/Blueprints/BPC_RPGSystem.bIsDead` (`self.BPC_RPGSystem_AI`))
        _
        (elif (and (> Last (`/Game/RPGSystem/Blueprints/BPC_RPGSystem.GetResourceType` (`self.BPC_RPGSystem_AI`) Type)) (!= Last 0.0))
          (`/Engine/EditorBlueprintResources/StandardMacros.IsValid` (`self.HealthBar`)
            (:`Is Valid`
              _)
            (:`Is Not Valid`
              (`/Engine/EditorBlueprintResources/StandardMacros.IsValid` _mesh
                (:`Is Valid`
                  (bind _returnvalue (`AddComponent|NODE_AddWidgetComponent-0` :`RelativeTransform` (`KismetMathLibrary.MakeTransform` (`KismetMathLibrary.MakeVector` 0.0 0.0 (* (.z (`.BoxExtent` (`KismetSystemLibrary.GetComponentBounds` _mesh))) 1.0)))))
                  (set `self.HealthBar` _returnvalue)))))
          (message `/Game/RPGSystem/Blueprints/Utilities/BPI_RPG_NamePlate.UpdateInfoHP` (`WidgetComponent.GetUserWidgetObject` (`self.HealthBar`)) (`/Game/RPGSystem/Blueprints/BPC_RPGSystem.GetResourceType` _bpc_rpgsystem_ai_2 "NewEnumerator0") (`.Percent` (`/Game/RPGSystem/Blueprints/BPC_RPGSystem.GetStatBonus` _bpc_rpgsystem_ai_2 "NewEnumerator13"))))))
    (:`NewEnumerator1`
      (`/Engine/EditorBlueprintResources/StandardMacros.IsValid` (`self.HealthBar`)
        (:`Is Valid`
          (message `/Game/RPGSystem/Blueprints/Utilities/BPI_RPG_NamePlate.UpdateInfoSP` (`WidgetComponent.GetUserWidgetObject` (`self.HealthBar`)) (`/Game/RPGSystem/Blueprints/BPC_RPGSystem.GetResourceType` _bpc_rpgsystem_ai "NewEnumerator1") (`.Percent` (`/Game/RPGSystem/Blueprints/BPC_RPGSystem.GetStatBonus` _bpc_rpgsystem_ai "NewEnumerator18"))))))))

(event `self.ReceiveBeginPlay`
  (bind _bpc_rpgsystem_ai (`self.BPC_RPGSystem_AI`))
  ;[1 1 1] BeginPlay - Major Update 3 - Changed
  (`|ExecutionSequence`
    (:`then_0`
      (add `/Game/RPGSystem/Blueprints/BPC_RPGSystem.OnDeath` (`self.BPC_RPGSystem_AI`) (`|CreateDelegate` :!event `OnDead`))
      (add `/Game/RPGSystem/Blueprints/BPC_RPGSystem.OnCompanionInit` _bpc_rpgsystem_ai (`|CreateDelegate` :!event `CreateHealthBar`))
      (add `/Game/RPGSystem/Blueprints/BPC_RPGSystem.OnMinionInit` _bpc_rpgsystem_ai (`|CreateDelegate` :!event `CreateHealthBar`))
      (add `/Game/RPGSystem/Blueprints/BPC_RPGSystem.OnResourceTypeChanged` (`self.BPC_RPGSystem_AI`) (`|CreateDelegate` :!event `OnResourceTypeChanged`)))
    (:`then_1`
      (`self.SetActorTickEnabled` true))))

(event `CreateHealthBar`
  (bind _followerfloatinghud_owneronly (`self.FollowerFloatingHUD_OwnerOnly`))
  (bind _followertype (`/Game/RPGSystem/Blueprints/BPC_RPGSystem.FollowerType` (`self.BPC_RPGSystem_AI`)))
  (bind _returnvalue (== (`ActorComponent.GetOwner` (`/Game/RPGSystem/Blueprints/BPC_RPGSystem.FollowerMaster` (`self.BPC_RPGSystem_AI`))) (`GameplayStatics.GetPlayerCharacter` 0)))
  ;[1 1 1] BeginPlay - Major Update 3 - Changed
  (`/Engine/EditorBlueprintResources/StandardMacros.IsValid` (`self.HealthBar`)
    (:`Is Not Valid`
      (if (`|EnumEquality` _followertype "NewEnumerator2")
        (if _followerfloatinghud_owneronly
          (`/Engine/EditorBlueprintResources/StandardMacros.IsValid` (`GameplayStatics.GetPlayerCharacter` 0)
            (:`Is Valid`
              (if _returnvalue
                (bind _returnvalue_2 (`AddComponent|NODE_AddWidgetComponent-1` :`RelativeTransform` (`KismetMathLibrary.MakeTransform` (`KismetMathLibrary.MakeVector` 0.0 0.0 (* (.z (`.BoxExtent` (`KismetSystemLibrary.GetComponentBounds` (`self.Mesh`)))) 1.75))) :!label _label))
                (set `self.HealthBar` _returnvalue_2))))
          (else
            (goto _label)))
        (elif (`|EnumEquality` _followertype "NewEnumerator1")
          (if _followerfloatinghud_owneronly
            (`/Engine/EditorBlueprintResources/StandardMacros.IsValid` (`GameplayStatics.GetPlayerCharacter` 0)
              (:`Is Valid`
                (if _returnvalue
                  (bind _returnvalue_3 (`AddComponent|NODE_AddWidgetComponent-2` :`RelativeTransform` (`KismetMathLibrary.MakeTransform` (`KismetMathLibrary.MakeVector` 0.0 0.0 (* (.z (`.BoxExtent` (`KismetSystemLibrary.GetComponentBounds` (`self.Mesh`)))) 1.0))) :!label _label_2))
                  (set `self.HealthBar` _returnvalue_3))))
            (else
              (goto _label_2))))))))

(event `self.ReceiveDestroyed`
  (bind _healthbar (`self.HealthBar`))
  ;[1 1 1] Destroyed
  (`/Engine/EditorBlueprintResources/StandardMacros.IsValid` _healthbar
    (:`Is Valid`
      (`ActorComponent.K2_DestroyComponent` _healthbar))))

(event `/Game/RPGSystem/Blueprints/Utilities/BPI_RPG_Interaction.SelectInteractable`
  (params (Selected :type Boolean))
  (bind _mesh (`self.Mesh`))
  ;[1 1 1] Select Interactable
  (`/Engine/EditorBlueprintResources/StandardMacros.IsValid` _mesh
    (:`Is Valid`
      (`PrimitiveComponent.SetRenderCustomDepth` _mesh Selected))))

(event `/Game/RPGSystem/Blueprints/Utilities/BPI_RPG_PlayerCharacter.VE_DestroyComponent`
  (params (Component :type "ActorComponent Object Reference"))
  ;[1 1 1] Visual Equipment
  (`ActorComponent.K2_DestroyComponent` Component))

(event `self.VisualEquipmentDestroyComponents`
  (params (Components :type "Array of ActorComponent Object Reference (by ref)"))
  ;[1 1 1] Visual Equipment
  (`ActorComponent.K2_DestroyComponent` Components))

(event `self.ReceiveUnpossessed`
  (params (OldController :type "Controller Object Reference"))
  ;[1 1 1] BeginPlay - Major Update 3 - Changed
  (`self.SetLifeSpan` OldController 0.01))

(event `ActivateRagdoll`
  (params (Impulse_Struct :type "/Game/RPGSystem/Blueprints/Structure/Skill/S_ImpactInfo Structure"))
  (bind _capsulecomponent (`self.CapsuleComponent`))
  ;[1 1 1] Ragdoll
  (bind _bones (`/Game/RPGSystem/Blueprints/Utilities/BPI_RPG_PlayerCharacter.GetBonesForImpulse`))
  (bind _force (`self.GetRagdollForceMultiplier`))
  (`/Game/RPGSystem/Blueprints/BPC_RPGSystem.EnableRagdoll` (`self.BPC_RPGSystem_AI`) (`self.Mesh`) Impulse_Struct _bones _force)
  (`ActorComponent.Deactivate` (`self.CharacterMovement`))
  (`ActorComponent.Deactivate` (`self.BPC_RPGSystem_AI`))
  (`ActorComponent.Deactivate` (`self.CapsuleComponent`))
  (`ActorComponent.SetComponentTickEnabled` (`self.BPC_RPGSystem_AI`) false)
  (`ActorComponent.SetComponentTickEnabled` (`self.CharacterMovement`) false)
  (`self.SetActorTickInterval` 1.0)
  (set `self.DeathTime` (`KismetSystemLibrary.GetGameTimeInSeconds`))
  (set `self.MakeRagdollChecks` true)
  (`KismetSystemLibrary.Delay` 0.15)
  (`/Game/RPGSystem/Blueprints/BPC_RPGSystem.SetVisualEquipmentSimulate` (`self.BPC_RPGSystem_AI`) true)
  (`/Engine/EditorBlueprintResources/StandardMacros.IsValid` _capsulecomponent
    (:`Is Valid`
      (`ActorComponent.K2_DestroyComponent` _capsulecomponent))))

(event `OnDead`
  (params (Attacker :type "/Game/RPGSystem/Blueprints/BPC_RPGSystem Object Reference") (Impulse :type "/Game/RPGSystem/Blueprints/Structure/Skill/S_ImpactInfo Structure") (Victim :type "/Game/RPGSystem/Blueprints/BPC_RPGSystem Object Reference"))
  (bind _bpc_rpgsystem_ai (`self.BPC_RPGSystem_AI`))
  ;[1 1 1] OnDeath
  (`/Engine/EditorBlueprintResources/StandardMacros.IsValid` (`self.HealthBar`)
    (:`Is Valid`
      (`ActorComponent.K2_DestroyComponent` (`self.HealthBar`)))
    (:`Is Not Valid`
      _))
  (`/Game/RPGSystem/Blueprints/BPC_RPGSystem.InterruptCast` _bpc_rpgsystem_ai)
  (`ActorComponent.SetComponentTickEnabled` _bpc_rpgsystem_ai false)
  (`/Engine/EditorBlueprintResources/ActorMacros.Switch Has Authority`
    (:`Authority`
      (`Controller.UnPossess` (`self.GetController`)))
    (:`Remote`
      _))
  (`NavMovementComponent.StopActiveMovement` (`self.CharacterMovement`))
  (`self.ActivateRagdoll` Impulse))

(event `/Game/RPGSystem/Blueprints/Utilities/BPI_RPG_Animation.SetAnimationState`
  (params (State :type "/Game/RPGSystem/Blueprints/Enum/Item/E_Item_WeaponType Enum" :default "NewEnumerator0"))
  ;[1 1 1] Animations
  (set `self.AnimationState` State))

(event `/Game/RPGSystem/Blueprints/Utilities/BPI_RPG_Animation.PlayHitAnimation`
  (params (Impulse :type "/Game/RPGSystem/Blueprints/Structure/Skill/S_ImpactInfo Structure"))
  ;[1 1 1] Animations
  (message `/Game/RPGSystem/Blueprints/Utilities/BPI_RPG_Animation.PlayHitAnimation` (`SkeletalMeshComponent.GetAnimInstance` (`self.Mesh`)) Impulse))

(event `self.ReceiveTick`
  (params (DeltaSeconds :type "Float (single-precision)"))
  (bind _mesh (`self.Mesh`))
  (bind _returnvalue (`/Game/RPGSystem/Blueprints/BPC_RPGSystem.GetCrowdControl` (`self.BPC_RPGSystem_AI`) "NewEnumerator8"))
  (bind _bisdead (`/Game/RPGSystem/Blueprints/BPC_RPGSystem.bIsDead` (`self.BPC_RPGSystem_AI`)))
  ;[1 1 1] Smooth Rotation
  (if (`KismetSystemLibrary.IsServer`)
    (if _bisdead
      ;[1 1 1] Convert to poseable | using tick since "LifeSpan" also uses a tick in background, we so can do that here instead
      (if (and (`self.MakeRagdollChecks`) (> (- (`KismetSystemLibrary.GetGameTimeInSeconds`) (`self.DeathTime`)) 3.0)) :!label _label_3
        (if (`self.PoseableSpawned`)
          (if (or (not (`PrimitiveComponent.WasRecentlyRendered` (`self.PoseableRagdoll`) 0.1)) (> (- (`KismetSystemLibrary.GetGameTimeInSeconds`) (`self.DeathTime`)) (`self.MaxDeath_Lifetime`)))
            (`self.K2_DestroyActor`))
          (elif (<= (`KismetMathLibrary.VSize` (`SceneComponent.GetComponentVelocity` (`self.Mesh`))) 5.0)
            ;[1 1 1] Spawn poseable and remove Mesh
            (bind _returnvalue_2 (`AddComponent|NODE_AddPoseableMeshComponent-1` :`RelativeTransform` (`SceneComponent.GetRelativeTransform` _mesh)))
            (set `self.PoseableRagdoll` _returnvalue_2)
            (`SkinnedMeshComponent.SetSkinnedAssetAndUpdate` _returnvalue_2 (`SkinnedMeshComponent.GetSkinnedAsset` _mesh) false)
            (for _array_element (`SceneComponent.GetAllSocketNames` _mesh)
              (`PoseableMeshComponent.SetBoneTransformByName` _returnvalue_2 _array_element (`SceneComponent.GetSocketTransform` (`self.Mesh`) _array_element "RTS_World") "WorldSpace"))
            (`ActorComponent.K2_DestroyComponent` _mesh)
            (set `self.PoseableSpawned` true)
            (`/Game/RPGSystem/Blueprints/BPC_RPGSystem.SetVisualEquipmentSimulate` (`self.BPC_RPGSystem_AI`) false))))
      (else
        (if _returnvalue
          (`|ExecutionSequence`
            (:`then_0`
              (`/Engine/EditorBlueprintResources/StandardMacros.Gate` false :!label _label_4
                (:`Exit`
                  (`MovementComponent.StopMovementImmediately` (`self.CharacterMovement`))
                  (goto _label_4 :!via `Close`))))
            (:`then_1`
              _))
          (else
            (`|ExecutionSequence`
              (:`then_0`
                _)
              (:`then_1`
                (goto _label_4 :!via `Open`)))))
        (if (not _returnvalue)
          (`/Engine/EditorBlueprintResources/StandardMacros.IsValid` (`AIBlueprintHelperLibrary.GetAIController` self)
            (:`Is Valid`
              (if (> (`KismetMathLibrary.VSize` (`CharacterMovementComponent.GetLastUpdateVelocity` (`self.CharacterMovement`))) 5.0)
                (set `CharacterMovementComponent.bOrientRotationToMovement` true (`self.CharacterMovement`))
                (else
                  (set `CharacterMovementComponent.bOrientRotationToMovement` false (`self.CharacterMovement`))))
              (if (`.AllowStrafe_327_496D2391412F4F8C1278E2BB3556597E` (break `/Game/RPGSystem/Blueprints/Structure/Monster/S_Monster` (`/Game/RPGSystem/Blueprints/BPC_RPGSystem_AI.EnemyInfo` (`self.BPC_RPGSystem_AI`))))
                _))))))
    (elif _bisdead
      (goto _label_3))))

(event `/Game/RPGSystem/Blueprints/Utilities/BPI_RPG_Animation.PlaySkillAnimation`
  (params (`State ` :type "/Game/RPGSystem/Blueprints/Enum/Skill/E_SkillAnimationState Enum" :default "NewEnumerator3") (`SkillID ` :type Name) (PlayRate :type "Float (double-precision)") (CCD_Ratio :type "Float (double-precision)") (Time :type "Float (double-precision)") (Message :type String))
  (bind _mesh (`self.Mesh`))
  ;[1 1 1] Animations
  (if (`KismetSystemLibrary.IsValid` _mesh)
    (message `/Game/RPGSystem/Blueprints/Utilities/BPI_RPG_Animation.PlaySkillAnimation` (`SkeletalMeshComponent.GetAnimInstance` _mesh) `State ` `SkillID ` PlayRate CCD_Ratio Time Message)))

(event `/Game/RPGSystem/Blueprints/Utilities/BPI_RPG_Animation.StopSkillAnimation`
  ;[1 1 1] Animations
  (`self.StopAnimMontage` (`self.GetCurrentMontage`)))

(fn `Get Skeletal Mesh`
  (returns (Success :type Boolean) (Component :type "SkeletalMeshComponent Object Reference"))
  (bind _mesh (`self.Mesh`))
  (return (`KismetSystemLibrary.IsValid` _mesh) _mesh))

(fn `GetAnimationState`
  (returns (State :type "/Game/RPGSystem/Blueprints/Enum/Item/E_Item_WeaponType Enum"))
  (return (`self.AnimationState`)))

(fn `GetBonesForImpulse`
  (returns (Bones :type "Array of Name"))
  (return (`|MakeArray` (`SkinnedMeshComponent.GetBoneName` (`self.Mesh`) 0))))

(fn `GetCharacterMovementComponent`
  (returns (Component :type "CharacterMovementComponent Object Reference"))
  (return null))

(fn `GetCurrentSkillAnimationCCD_Ratio`
  (returns (Return :type "Float (double-precision)"))
  (return 0.0))

(fn `GetCurrentSkillAnimationPlayRate`
  (returns (Return :type "Float (double-precision)"))
  (return 0.0))

(fn `GetDropSystemComponent`
  (returns (Success :type Boolean) (Component :type "/Game/RPGSystem/Blueprints/BPC_DropSystem Object Reference"))
  (return true (`self.BPC_DropSystem`)))

(fn `GetEnemyInfo`
  (returns (Succes :type Boolean) (MonsterID :type Name) (Info :type "/Game/RPGSystem/Blueprints/Structure/Monster/S_Monster Structure") (CustomVariables :type "/Game/RPGSystem/Blueprints/Structure/Misc/S_ArrayOf_FName Structure") (CustomVariablesPrivate :type "/Game/RPGSystem/Blueprints/Structure/Misc/S_ArrayOf_FName Structure"))
  (locals (VarCustomVariables :type "Array of Name") (VarCustomVariablesPrivate :type "Array of Name"))
  (bind _bpc_rpgsystem_ai (`self.BPC_RPGSystem_AI`))
  (bind _bpc_rpgsystem_ai_2 (`self.BPC_RPGSystem_AI`))
  (set `local.VarCustomVariables` (`/Game/RPGSystem/Blueprints/BPC_RPGSystem_AI.CustomVariables` _bpc_rpgsystem_ai))
  (set `local.VarCustomVariablesPrivate` (`/Game/RPGSystem/Blueprints/BPC_RPGSystem_AI.CustomVariablesPrivate` _bpc_rpgsystem_ai))
  (for _array_element (`/Game/RPGSystem/Blueprints/BPC_RPGSystem_AI.CustomVariablesTags` (`self.BPC_RPGSystem_AI`))
    (`KismetArrayLibrary.Array_Add` (`local.VarCustomVariables`) (`BlueprintGameplayTagLibrary.GetTagName` _array_element)))
  (for _array_element_2 (`/Game/RPGSystem/Blueprints/BPC_RPGSystem_AI.CustomVariablesTagsPrivate` (`self.BPC_RPGSystem_AI`))
    (`KismetArrayLibrary.Array_Add` (`local.VarCustomVariablesPrivate`) (`BlueprintGameplayTagLibrary.GetTagName` _array_element_2)))
  (return true (`/Game/RPGSystem/Blueprints/BPC_RPGSystem_AI.MonsterID` _bpc_rpgsystem_ai_2) (`/Game/RPGSystem/Blueprints/BPC_RPGSystem_AI.EnemyInfo` _bpc_rpgsystem_ai_2) (make `/Game/RPGSystem/Blueprints/Structure/Misc/S_ArrayOf_FName` (`local.VarCustomVariables`)) (make `/Game/RPGSystem/Blueprints/Structure/Misc/S_ArrayOf_FName` (`local.VarCustomVariablesPrivate`))))

(fn `GetInteractableComponents`
  (returns (Components :type "Array of PrimitiveComponent Object Reference"))
  (return))

(fn `GetInteractInfo`
  (params (Player :type "/Game/RPGSystem/Blueprints/BPC_RPGSystem Object Reference"))
  (returns (Success :type Boolean) (Type :type "/Game/RPGSystem/Blueprints/Enum/Interact/E_InteractType Enum") (Action :type "/Game/RPGSystem/Blueprints/Enum/Interact/E_InteractAction Enum"))
  (bind _player (`local.Player`))
  (bind _returnvalue (`ActorComponent.GetOwner` (`local.Player`)))
  (bind _returnvalue_2 (`self.K2_GetActorLocation` _returnvalue))
  ;[1 1 1] Define Outline color index
  (if (`/Game/RPGSystem/Blueprints/BPC_RPGSystem.bIsDead` (`self.BPC_RPGSystem_AI`))
    (return false "NewEnumerator1" "NewEnumerator9")
    (else
      (bind _return (`self.IsDamageable` (`/Game/RPGSystem/Blueprints/BPC_RPGSystem.TeamID` Player)))
      (if _return
        (`PrimitiveComponent.SetCustomDepthStencilValue` (`self.Mesh`) 1)
        (bind (_radius _halfheight) (message `/Game/RPGSystem/Blueprints/Utilities/BPI_RPG_PlayerCharacter.GetMeshRadius` (`ActorComponent.GetOwner` _player)))
        (bind _worldlocation (`self.GetMoveToEndDestination` (`local.Player`)))
        (bind _return_2 (`self.GetLookAtLocation`))
        (if (<= (`/Game/RPGSystem/Blueprints/Utilities/BPL_RPG_Utilities.GetDistanceExt` _returnvalue_2 _worldlocation _radius _halfheight) (* (`/Game/RPGSystem/Blueprints/BPC_RPGSystem.GetSkillAttackRangeUnits` _player) 0.9))
          (if (`/Game/RPGSystem/Blueprints/Utilities/BPL_RPG_Utilities.IsTargetInAngle` _return_2 _returnvalue_2 (`self.GetActorForwardVector` _returnvalue) (* (`CapsuleComponent.GetScaledCapsuleRadius` (`self.CapsuleComponent`)) 0.75))
            (return true "NewEnumerator1" "NewEnumerator8")
            (else
              (return true "NewEnumerator1" "NewEnumerator5")))
          (else
            (return true "NewEnumerator1" "NewEnumerator1")))
        (else
          (`PrimitiveComponent.SetCustomDepthStencilValue` (`self.Mesh`) 2)
          (return true "NewEnumerator0" "NewEnumerator9"))))))

(fn `GetLookAtLocation`
  (returns (Return :type "Vector Structure"))
  (return (`self.K2_GetActorLocation`)))

(fn `GetMeshRadius`
  (returns (Radius :type "Float (double-precision)") (HalfHeight :type "Float (double-precision)"))
  (bind _capsulecomponent (`self.CapsuleComponent`))
  (if (`KismetSystemLibrary.IsValid` _capsulecomponent)
    (return (* (`CapsuleComponent.GetScaledCapsuleRadius` _capsulecomponent) 1.0) 0.0)
    (else
      (return 0.0 0.0))))

(fn `GetMovementSpeed`
  (returns (Speed :type "Float (double-precision)"))
  (return (`CharacterMovementComponent.MaxWalkSpeed` (`self.CharacterMovement`))))

(fn `GetMoveToEndDestination`
  (params (Player :type "/Game/RPGSystem/Blueprints/BPC_RPGSystem Object Reference"))
  (returns (WorldLocation :type "Vector Structure"))
  (return (`self.K2_GetActorLocation`)))

(fn `GetRagdollForceMultiplier`
  (returns (Force :type "Float (double-precision)"))
  (return 1.0))

(fn `GetRPGSystem`
  (returns (Success :type Boolean) (Reference :type "/Game/RPGSystem/Blueprints/BPC_RPGSystem Object Reference"))
  (bind _bpc_rpgsystem_ai (`self.BPC_RPGSystem_AI`))
  (return (`KismetSystemLibrary.IsValid` _bpc_rpgsystem_ai) _bpc_rpgsystem_ai))

(fn `GetRPGSystemAI`
  (returns (Success :type Boolean) (Reference :type "/Game/RPGSystem/Blueprints/BPC_RPGSystem_AI Object Reference"))
  (bind _bpc_rpgsystem_ai (`self.BPC_RPGSystem_AI`))
  (return (`KismetSystemLibrary.IsValid` _bpc_rpgsystem_ai) _bpc_rpgsystem_ai))

(fn `GetScreenTooltipInfo`
  (params (Player :type "/Game/RPGSystem/Blueprints/BPC_RPGSystem Object Reference")))

(fn `GetTeamID`
  (returns (Return :type String))
  (return ""))

(fn `GetWorldTooltipInfo`
  (params (HitComp :type "PrimitiveComponent Object Reference"))
  (returns (Success :type Boolean) (Interactable :type Boolean) (Text :type Text) (Color :type "LinearColor Structure") (Offset :type "Vector Structure"))
  (return false false "" (struct) (0.0 0.0 0.0)))

(fn `IsDamageable`
  (params (TeamID :type String))
  (returns (Return :type Boolean))
  (return (`KismetStringLibrary.NotEqual_StrStr` TeamID (`/Game/RPGSystem/Blueprints/BPC_RPGSystem.TeamID` (`self.BPC_RPGSystem_AI`)))))

(fn `IsDualWield`
  (returns (Success :type Boolean))
  (bind _bpc_rpgsystem_ai (`self.BPC_RPGSystem_AI`))
  (`/Engine/EditorBlueprintResources/StandardMacros.IsValid` _bpc_rpgsystem_ai
    (:`Is Valid`
      (return (`/Game/RPGSystem/Blueprints/BPC_RPGSystem.IsDualWield` _bpc_rpgsystem_ai)))
    (:`Is Not Valid`
      (return false))))

(fn `IsFalling`
  (returns (Falling :type Boolean))
  (return (`NavMovementComponent.IsFalling` (`self.CharacterMovement`))))

(fn `IsTwohanded`
  (returns (Success :type Boolean))
  (bind _bpc_rpgsystem_ai (`self.BPC_RPGSystem_AI`))
  (`/Engine/EditorBlueprintResources/StandardMacros.IsValid` _bpc_rpgsystem_ai
    (:`Is Valid`
      (return (`/Game/RPGSystem/Blueprints/BPC_RPGSystem.IsTwoHanded` _bpc_rpgsystem_ai)))
    (:`Is Not Valid`
      (return false))))

(fn `OptimizationTick`
  (locals (VarInRange :type Boolean))
  (bind _behaviortreecomp (`self.BehaviorTreeComp`))
  (bind _behaviortreecomp_2 (`self.BehaviorTreeComp`))
  (bind _returnvalue (`BrainComponent.IsRunning` _behaviortreecomp_2))
  (for _array_element (`GameStateBase.PlayerArray` (`GameplayStatics.GetGameState`))
    (`/Engine/EditorBlueprintResources/StandardMacros.IsValid` _array_element
      (:`Is Valid`
        (if (<= (`self.GetSquaredDistanceTo` self _array_element) 9000000.0)
          (set `local.VarInRange` true)
          (break)))))
  (`/Engine/EditorBlueprintResources/StandardMacros.IsValid` _behaviortreecomp_2
    (:`Is Valid`
      (if (`local.VarInRange`)
        (if (not _returnvalue)
          (`BrainComponent.StartLogic` _behaviortreecomp) ; Start Logic again
        )
        (elif _returnvalue
          (`BrainComponent.StopLogic` _behaviortreecomp "OutOfRange") ; Stop Logic
        )))))

(fn `PlayDespawnEffect`)

(fn `SetMeshRotation`
  (params (Target :type "Vector Structure (by ref)") (Rate :type "Float (double-precision)") (DeltaTime :type "Float (double-precision)"))
  (bind _mesh (`self.Mesh`))
  (bind _returnvalue (`SceneComponent.K2_GetComponentRotation` _mesh))
  (`SceneComponent.K2_SetWorldRotation` (`self.Mesh`) (`KismetMathLibrary.RInterpTo_Constant` _returnvalue (`KismetMathLibrary.ComposeRotators` (`KismetMathLibrary.MakeRotator` (.roll (`KismetMathLibrary.FindLookAtRotation` (`SceneComponent.K2_GetComponentLocation` _mesh) Target)) (.pitch _returnvalue) (.yaw (`KismetMathLibrary.FindLookAtRotation` (`SceneComponent.K2_GetComponentLocation` _mesh) Target))) (struct :`Yaw` -90.0)) DeltaTime (* Rate 100.0)) false true))

(fn `SetMovementSpeed`
  (params (ToDefault :type Boolean) (Speed :type "Float (double-precision)"))
  (set `CharacterMovementComponent.MaxWalkSpeed` (`KismetMathLibrary.SelectFloat` 600.0 Speed ToDefault) (`self.CharacterMovement`)))

(fn `UserConstructionScript`)