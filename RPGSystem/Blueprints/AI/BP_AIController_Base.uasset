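; Base AI controller for RPG enemies, companions and minions, running BT_Enemy and feeding its blackboard target, aggression, formation and skill.
; Pawn sensing and damage events pass through CheckTarget, which favours closer valid targets with a clear line trace unless forced.
; Masters and minions share targets through RPGSystem dispatchers, with randomised delays on receipt.
; Dispatchers are unbound and rebound to pause and resume target search.
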(event `/Game/RPGSystem/Blueprints/Utilities/BPI_RPG_AIController.ChangeSightRadius`
  (params (Radius :type "Float (double-precision)"))
  (bind _returnvalue (`AIBlueprintHelperLibrary.GetBlackboard` null))
  (bind _pawnsensing (`self.PawnSensing`))
  (bind _pawnsensing_2 (`self.PawnSensing`))
  ;[1 1 1] Change Sight Radius
  (if (> Radius 0.0)
    (set `PawnSensingComponent.SightRadius` Radius _pawnsensing)
    (set `PawnSensingComponent.bSeePawns` true _pawnsensing)
    (`ActorComponent.Activate` _pawnsensing false)
    (`PawnSensingComponent.SetSensingUpdatesEnabled` _pawnsensing true)
    (`BlackboardComponent.SetValueAsEnum` _returnvalue "AggressionState" 1)
    (else
      (set `PawnSensingComponent.SightRadius` 0.0 (`self.PawnSensing`))
      (set `PawnSensingComponent.bSeePawns` false _pawnsensing_2)
      (`PawnSensingComponent.SetSensingUpdatesEnabled` _pawnsensing_2 false)
      (`ActorComponent.Deactivate` _pawnsensing_2)
      (`BlackboardComponent.SetValueAsEnum` _returnvalue "AggressionState" 0))))

(event `OnMasterDeath`
  (params (Attacker :type "/Game/RPGSystem/Blueprints/BPC_RPGSystem Object Reference") (Impulse :type "/Game/RPGSystem/Blueprints/Structure/Skill/S_ImpactInfo Structure") (Victim :type "/Game/RPGSystem/Blueprints/BPC_RPGSystem Object Reference"))
  ;[1 1 1] OnMasterDeath
  (`BlackboardComponent.SetValueAsObject` (`self.BlackboardReference`) "MinionMaster" null)
  (`BlackboardComponent.SetValueAsEnum` (`self.BlackboardReference`) "FollowerType" 0))

(event `/Game/RPGSystem/Blueprints/Utilities/BPI_RPG_AIController.InitMinion`
  (bind _rpgsystem (`self.RPGSystem`))
  ;[1 1 1] SetIsSlave
  (bind (_success _reference) (message `/Game/RPGSystem/Blueprints/Utilities/BPI_RPG_PlayerCharacter.GetRPGSystem` (`BlackboardComponent.GetValueAsObject` (`AIBlueprintHelperLibrary.GetBlackboard` self) "MinionMaster")))
  (if _success
    (add `/Game/RPGSystem/Blueprints/BPC_RPGSystem.OnMinionMasterNewTarget` _reference (`|CreateDelegate` :!event `MasterNewTarget`))
    (if (or (`/Game/RPGSystem/Blueprints/BPC_RPGSystem.IsCompanion` _rpgsystem) (`/Game/RPGSystem/Blueprints/BPC_RPGSystem.IsMinion` _rpgsystem))
      (add `/Game/RPGSystem/Blueprints/BPC_RPGSystem.OnMovementSpeedChanged` _reference (`|CreateDelegate` :!event `OnMasterMovementSpeedChanged`))
      (else
        (add `/Game/RPGSystem/Blueprints/BPC_RPGSystem.OnDeath` _reference (`|CreateDelegate` :!event `OnMasterDeath`))))))

(event `/Game/RPGSystem/Blueprints/Utilities/BPI_RPG_AIController.InitAI_Controller`
  (bind ((`Aggro_275_3A5967C84B34FF33B6439ABF9D72EE4B` _aggro) (`AttackType_321_0B7EA5754102E7F1D20E90AD52D8B303` _attacktype) (`RangeType_319_4CD96F4C4DC103F1CC7E7AB12B07AD3F` _rangetype) (`DamageType_323_5421CABF4492EBF2C663F696D8ECC548` _damagetype) (`SightRadius_272_C39D81B4445B6208976C0B94479F77E2` _sightradius)) (break `/Game/RPGSystem/Blueprints/Structure/Monster/S_Monster` (`/Game/RPGSystem/Blueprints/BPC_RPGSystem_AI.EnemyInfo` (`self.RPGSystem`))))
  ;[1 1 1] Init Ai Controller
  (`|ExecutionSequence`
    (:`then_0`
      (`self.ChangeSightRadius` (`KismetMathLibrary.SelectFloat` _sightradius 0.0 _aggro)))
    (:`then_1`
      (`BlackboardComponent.SetValueAsEnum` (`AIBlueprintHelperLibrary.GetBlackboard` self) "AIState" (`/Game/RPGSystem/Blueprints/BPC_RPGSystem.AI State` (`self.RPGSystem`))))))

(event `self.ReceivePossess`
  (params (PossessedPawn :type "Pawn Object Reference"))
  (bind _returnvalue (`AIBlueprintHelperLibrary.GetBlackboard` self))
  ;[1 1 1] On Possess
  (`|ExecutionSequence`
    (:`then_0`
      (`self.RunBehaviorTree` "/Game/RPGSystem/Blueprints/AI/BT_Enemy.BT_Enemy")
      (`/Engine/EditorBlueprintResources/StandardMacros.IsValid` _returnvalue
        (:`Is Valid`
          (set `self.BlackboardReference` _returnvalue)
          (bind (_success _reference) (message `/Game/RPGSystem/Blueprints/Utilities/BPI_RPG_PlayerCharacter.GetRPGSystemAI` PossessedPawn))
          (if _success
            (bind _output_get (set `self.RPGSystem` _reference))
            (add `/Game/RPGSystem/Blueprints/BPC_RPGSystem.OnDamageTaken` _output_get (`|CreateDelegate` :!event `OnDamageTaken`))
            (if (`/Game/RPGSystem/Blueprints/BPC_RPGSystem.IsCompanion` (`self.RPGSystem`))
              _)))))
    (:`then_1`
      (`KismetSystemLibrary.Delay` 0.25)
      (set `self.CanFindTarget` true))))

(event `MasterNewTarget`
  (params (NewTarget :type "/Game/RPGSystem/Blueprints/BPC_RPGSystem Object Reference"))
  (bind _returnvalue (`ActorComponent.GetOwner` NewTarget))
  (bind _rpgsystem (`self.RPGSystem`))
  (bind _returnvalue_2 (`AIBlueprintHelperLibrary.GetBlackboard` self))
  (bind _followermaster (`/Game/RPGSystem/Blueprints/BPC_RPGSystem.FollowerMaster` (`self.RPGSystem`)))
  ;[1 1 1] Slave New Target from Master
  (`KismetSystemLibrary.Delay` (`KismetMathLibrary.RandomFloatInRange` 0.2 1.2)) ; Do add some randomness
  (`/Engine/EditorBlueprintResources/StandardMacros.IsValid` NewTarget
    (:`Is Valid`
      (`/Engine/EditorBlueprintResources/StandardMacros.IsValid` _returnvalue_2
        (:`Is Valid`
          (if (!= (`BlackboardComponent.GetValueAsObject` _returnvalue_2 "MinionMaster") NewTarget)
            (if (or (`/Game/RPGSystem/Blueprints/BPC_RPGSystem.IsCompanion` _rpgsystem) (`/Game/RPGSystem/Blueprints/BPC_RPGSystem.IsMinion` _rpgsystem))
              (if (not (`BlackboardComponent.GetValueAsBool` _returnvalue_2 "HasTarget"))
                (`BlackboardComponent.SetValueAsObject` _returnvalue_2 "Target" _returnvalue :!label _label)
                (`BlackboardComponent.SetValueAsBool` _returnvalue_2 "HasTarget" true)
                (`BlackboardComponent.SetValueAsVector` _returnvalue_2 "TargetLocation" (`self.K2_GetActorLocation` _returnvalue))
                (`/Engine/EditorBlueprintResources/StandardMacros.IsValid` _followermaster
                  (:`Is Valid`
                    (remove `/Game/RPGSystem/Blueprints/BPC_RPGSystem.OnMinionMasterNewTarget` _followermaster (`|CreateDelegate` :!event `MasterNewTarget`)))))
              (else
                (goto _label)))))))))

(event `/Game/RPGSystem/Blueprints/Utilities/BPI_RPG_AIController.InitMaster`
  ;[1 1 1] Comment
  (`/Engine/EditorBlueprintResources/StandardMacros.IsValid` (`self.RPGSystem`)
    (:`Is Valid`
      (add `/Game/RPGSystem/Blueprints/BPC_RPGSystem.OnMinionNewTarget` (`self.RPGSystem`) (`|CreateDelegate` :!event `MinionNewTarget`))
      (`BlackboardComponent.SetValueAsBool` (`AIBlueprintHelperLibrary.GetBlackboard` null) "IsMaster" true))))

(event `OnMasterMovementSpeedChanged`
  (params (Speed :type "Float (double-precision)"))
  (bind _returnvalue (`self.K2_GetPawn`))
  ;[1 1 1] On Master Movementspeed changed | Companion/Minion
  (bind _speed (message `/Game/RPGSystem/Blueprints/Utilities/BPI_RPG_PlayerCharacter.GetMovementSpeed` _returnvalue))
  (message `/Game/RPGSystem/Blueprints/Utilities/BPI_RPG_PlayerCharacter.SetMovementSpeed` _returnvalue false (`KismetMathLibrary.SelectFloat` Speed _speed (> Speed _speed))))

(event `self.PawnSensing.OnSeePawn`
  (params (Pawn :type "Pawn Object Reference"))
  ;[1 1 1] On See Pawn
  (bind (_success _reference) (message `/Game/RPGSystem/Blueprints/Utilities/BPI_RPG_PlayerCharacter.GetRPGSystem` Pawn))
  (if _success
    (`self.CheckTarget` _reference)))

(event `self.ReceiveUnPossess`
  (params (UnpossessedPawn :type "Pawn Object Reference"))
  ;[1 1 1] On Unpossess
  (`self.SetActorTickEnabled` false)
  (`self.K2_DestroyActor`))

(event `MinionNewTarget`
  (params (NewParam :type "/Game/RPGSystem/Blueprints/BPC_RPGSystem Object Reference"))
  (bind _returnvalue (`ActorComponent.GetOwner` NewParam))
  (bind _rpgsystem (`self.RPGSystem`))
  (bind _returnvalue_2 (`AIBlueprintHelperLibrary.GetBlackboard` self))
  ;[1 1 1] Master new target from Slave
  (`KismetSystemLibrary.Delay` (`KismetMathLibrary.RandomFloatInRange` 0.5 1.0)) ; Do add some randomness
  (`/Engine/EditorBlueprintResources/StandardMacros.IsValid` NewParam
    (:`Is Valid`
      (`/Engine/EditorBlueprintResources/StandardMacros.IsValid` _returnvalue_2
        (:`Is Valid`
          (`/Engine/EditorBlueprintResources/StandardMacros.IsValid` (`BlackboardComponent.GetValueAsObject` _returnvalue_2 "Target")
            (:`Is Not Valid`
              (if (!= NewParam (`self.RPGSystem`))
                (`BlackboardComponent.SetValueAsObject` _returnvalue_2 "Target" _returnvalue)
                (`BlackboardComponent.SetValueAsBool` _returnvalue_2 "HasTarget" true)
                (`BlackboardComponent.SetValueAsVector` _returnvalue_2 "TargetLocation" (`self.K2_GetActorLocation` _returnvalue))
                (`/Game/RPGSystem/Blueprints/BPC_RPGSystem.OnMinionMasterNewTarget` _rpgsystem NewParam)
                (`/Game/RPGSystem/Blueprints/BPC_RPGSystem.OnMinionFollowMe` _rpgsystem)
                (remove `/Game/RPGSystem/Blueprints/BPC_RPGSystem.OnMinionNewTarget` (`self.RPGSystem`) (`|CreateDelegate` :!event `MinionNewTarget`))))))))))

(event `OnDamageTaken`
  (params (Attacker :type "/Game/RPGSystem/Blueprints/BPC_RPGSystem Object Reference") (Damage :type "Float (double-precision)") (DamageTo :type "/Game/RPGSystem/Blueprints/Enum/Basic/E_ResourceType Enum" :default "NewEnumerator0") (Element :type "/Game/RPGSystem/Blueprints/Enum/Basic/E_Element Enum" :default "NewEnumerator7") (Impulse :type "/Game/RPGSystem/Blueprints/Structure/Skill/S_ImpactInfo Structure") (IsSE :type Boolean) (ID :type Name))
  ;[1 1 1] OnDamageTaken
  (`self.CheckTarget` Attacker))

(event `/Game/RPGSystem/Blueprints/Utilities/BPI_RPG_AIController.SearchNewTarget`
  (bind _pawnsensing (`self.PawnSensing`))
  ;[1 1 1] Search for new target and re-enabling the dispatchers
  (`self.EnableDispatchers`)
  (`PawnSensingComponent.SetSensingInterval` _pawnsensing 0.01)
  (`PawnSensingComponent.SetSensingUpdatesEnabled` _pawnsensing true)
  (`KismetSystemLibrary.Delay` 0.2)
  (`PawnSensingComponent.SetSensingInterval` (`self.PawnSensing`) (`KismetMathLibrary.RandomFloatInRange` 0.2 1.5)))

(event `/Game/RPGSystem/Blueprints/Utilities/BPI_RPG_AIController.DisableTargetSearchForDuration`
  (params (Duration :type "Float (double-precision)"))
  ;[1 1 1] Disable Target Search For Duration
  (set `self.CanFindTarget` false)
  (`self.DisableDispatchers`)
  (`KismetSystemLibrary.RetriggerableDelay` Duration)
  (set `self.CanFindTarget` true)
  (`self.EnableDispatchers`))

(event `/Game/RPGSystem/Blueprints/Utilities/BPI_RPG_AIController.DisableTargetSearchUntilInRangeOfMaster`
  (bind _returnvalue (`self.K2_GetPawn`))
  (bind _followermaster (`/Game/RPGSystem/Blueprints/BPC_RPGSystem.FollowerMaster` (`self.RPGSystem`)))
  ;[1 1 1] Disable Target Search until in range of Master
  (if (!= (`KismetMathLibrary.Conv_ByteToInt` (`BlackboardComponent.GetValueAsEnum` (`AIBlueprintHelperLibrary.GetBlackboard` null) "FollowerType")) 0)
    (set `self.CanFindTarget` false)
    (`self.DisableDispatchers`)
    (`KismetSystemLibrary.Delay` 0.2 :!label _label_2)
    (`/Engine/EditorBlueprintResources/StandardMacros.IsValid` _followermaster
      (:`Is Valid`
        (`/Engine/EditorBlueprintResources/StandardMacros.IsValid` _returnvalue
          (:`Is Valid`
            (if (<= (`KismetMathLibrary.Vector_Distance2D` (`self.K2_GetActorLocation` _returnvalue) (`self.K2_GetActorLocation` (`ActorComponent.GetOwner` _followermaster))) 500.0)
              _
              (else
                (goto _label_2))))
          (:`Is Not Valid`
            _)))
      (:`Is Not Valid`
        _))
    (set `self.CanFindTarget` true)
    (`self.EnableDispatchers`)))

(event `/Game/RPGSystem/Blueprints/Utilities/BPI_RPG_AIController.SetNewTarget`
  (params (Component :type "/Game/RPGSystem/Blueprints/BPC_RPGSystem Object Reference"))
  ;[1 1 1] Set new Target (Force)
  (`self.CheckTarget` Component true))

(event `/Game/RPGSystem/Blueprints/Utilities/BPI_RPG_AIController.SetAIState`
  (params (State :type "/Game/RPGSystem/Blueprints/Enum/Monster/E_AIState Enum" :default "NewEnumerator0"))
  (bind _rpgsystem (`self.RPGSystem`))
  ;[1 1 1] Set AI State
  (set `/Game/RPGSystem/Blueprints/BPC_RPGSystem.AI State` State _rpgsystem)
  (`BlackboardComponent.SetValueAsEnum` (`AIBlueprintHelperLibrary.GetBlackboard` self) "AIState" (`/Game/RPGSystem/Blueprints/BPC_RPGSystem.AI State` _rpgsystem)))

(event `/Game/RPGSystem/Blueprints/Utilities/BPI_RPG_AIController.SetAggressionState`
  (params (State :type "/Game/RPGSystem/Blueprints/Enum/Companion/E_CompanionAggressionState Enum" :default "NewEnumerator0"))
  (bind ((`Aggro_275_3A5967C84B34FF33B6439ABF9D72EE4B` _aggro) (`AttackType_321_0B7EA5754102E7F1D20E90AD52D8B303` _attacktype) (`RangeType_319_4CD96F4C4DC103F1CC7E7AB12B07AD3F` _rangetype) (`DamageType_323_5421CABF4492EBF2C663F696D8ECC548` _damagetype) (`SightRadius_272_C39D81B4445B6208976C0B94479F77E2` _sightradius)) (break `/Game/RPGSystem/Blueprints/Structure/Monster/S_Monster` (`/Game/RPGSystem/Blueprints/BPC_RPGSystem_AI.EnemyInfo` (`self.RPGSystem`))))
  ;[1 1 1] Set Aggression State
  (`BlackboardComponent.SetValueAsEnum` (`AIBlueprintHelperLibrary.GetBlackboard` null) "AggressionState" State)
  (switch `/Game/RPGSystem/Blueprints/Enum/Companion/E_CompanionAggressionState` State
    (:`NewEnumerator0`
      (`self.ChangeSightRadius` 0.0 :!label _label_3))
    (:`NewEnumerator1`
      (`self.ChangeSightRadius` (`KismetMathLibrary.SelectFloat` _sightradius 0.0 _aggro)))
    (:`NewEnumerator2`
      (goto _label_3))))

(event `/Game/RPGSystem/Blueprints/Utilities/BPI_RPG_AIController.SetFormationIndex`
  (params (Index :type Integer))
  ;[1 1 1] Set FormationIndex
  (`BlackboardComponent.SetValueAsInt` (`AIBlueprintHelperLibrary.GetBlackboard` null) "FormationIndex" Index))

(event `/Game/RPGSystem/Blueprints/Utilities/BPI_RPG_AIController.SetFormationType`
  (params (Formation :type "/Game/RPGSystem/Blueprints/Enum/Companion/E_CompanionFormationType Enum" :default "NewEnumerator0"))
  ;[1 1 1] Set FormationType
  (`BlackboardComponent.SetValueAsEnum` (`AIBlueprintHelperLibrary.GetBlackboard` null) "FormationType" Formation))

(event `/Game/RPGSystem/Blueprints/Utilities/BPI_RPG_AIController.SetSkillToUse`
  (params (SkillID :type Name))
  ;[1 1 1] Set Skill
  (`BlackboardComponent.SetValueAsName` (`AIBlueprintHelperLibrary.GetBlackboard` null) "SkillID" SkillID))

(event `/Game/RPGSystem/Blueprints/Utilities/BPI_RPG_AIController.SetMoveToLocation`
  (params (Location :type "Vector Structure"))
  (bind _returnvalue (`AIBlueprintHelperLibrary.GetBlackboard` null))
  ;[1 1 1] Set Move To Location
  (`self.DisableTargetSearchForDuration` 1.5)
  (`BlackboardComponent.SetValueAsObject` _returnvalue "Target" null)
  (`BlackboardComponent.SetValueAsBool` _returnvalue "HasTarget" false)
  (`BlackboardComponent.SetValueAsVector` _returnvalue "TargetLocation" Location)
  (`AIBlueprintHelperLibrary.SimpleMoveToLocation` null Location))

(event `/Game/RPGSystem/Blueprints/Utilities/BPI_RPG_AIController.ForgetTarget`
  (bind _returnvalue (`AIBlueprintHelperLibrary.GetBlackboard` self))
  ;[1 1 1] Forget Target
  (`BlackboardComponent.SetValueAsObject` _returnvalue "Target" null)
  (`BlackboardComponent.SetValueAsBool` _returnvalue "HasTarget" false)
  (`BlackboardComponent.SetValueAsVector` _returnvalue "TargetLocation" (0.0 0.0 0.0)))

(fn `CheckTarget`
  (params (Target :type "/Game/RPGSystem/Blueprints/BPC_RPGSystem Object Reference") (Force :type Boolean))
  (bind _returnvalue (`ActorComponent.GetOwner` Target))
  (bind _returnvalue_2 (`self.K2_GetPawn`))
  (bind _returnvalue_3 (`self.K2_GetPawn`))
  (bind _rpgsystem (`self.RPGSystem`))
  (bind _returnvalue_4 (`AIBlueprintHelperLibrary.GetBlackboard` self))
  (bind _returnvalue_5 (`AIBlueprintHelperLibrary.GetBlackboard` self))
  (if (`self.CanFindTarget`)
    (`/Engine/EditorBlueprintResources/StandardMacros.IsValid` Target
      (:`Is Valid`
        (`|ExecutionSequence`
          (:`then_0`
            (`/Engine/EditorBlueprintResources/StandardMacros.IsValid` _returnvalue_2
              (:`Is Valid`
                (if (`local.Force`)
                  (`BlackboardComponent.SetValueAsObject` _returnvalue_4 "Target" _returnvalue :!label _label)
                  (`BlackboardComponent.SetValueAsBool` _returnvalue_4 "HasTarget" true)
                  (`BlackboardComponent.SetValueAsVector` _returnvalue_4 "TargetLocation" (`self.K2_GetActorLocation` _returnvalue))
                  (remove `/Game/RPGSystem/Blueprints/BPC_RPGSystem.OnDamageTaken` (`self.RPGSystem`) (`|CreateDelegate` :!event `OnDamageTaken`))
                  (if (`BlackboardComponent.GetValueAsBool` (`AIBlueprintHelperLibrary.GetBlackboard` null) "IsMaster")
                    (`/Game/RPGSystem/Blueprints/BPC_RPGSystem.OnMinionMasterNewTarget` _rpgsystem Target)
                    (`/Game/RPGSystem/Blueprints/BPC_RPGSystem.OnMinionFollowMe` _rpgsystem)
                    (remove `/Game/RPGSystem/Blueprints/BPC_RPGSystem.OnMinionNewTarget` (`self.RPGSystem`) (`|CreateDelegate` :!event `MinionNewTarget`))
                    (else
                      (if (`|EnumEquality` (cast `/Game/RPGSystem/Blueprints/Enum/Companion/E_FollowerType` (`BlackboardComponent.GetValueAsEnum` (`AIBlueprintHelperLibrary.GetBlackboard` null) "FollowerType")) "NewEnumerator1")
                        (if (`KismetSystemLibrary.IsValid` (`/Game/RPGSystem/Blueprints/BPC_RPGSystem.FollowerMaster` (`self.RPGSystem`)))
                          (remove `/Game/RPGSystem/Blueprints/BPC_RPGSystem.OnMinionMasterNewTarget` (`/Game/RPGSystem/Blueprints/BPC_RPGSystem.FollowerMaster` (`self.RPGSystem`)) (`|CreateDelegate` :!event `MasterNewTarget`))))
                      (bind (_success _reference) (message `/Game/RPGSystem/Blueprints/Utilities/BPI_RPG_PlayerCharacter.GetRPGSystem` (`BlackboardComponent.GetValueAsObject` (`AIBlueprintHelperLibrary.GetBlackboard` self) "MinionMaster")))
                      (if _success
                        (`/Game/RPGSystem/Blueprints/BPC_RPGSystem.OnMinionNewTarget` _reference Target))))
                  (elif (`BlackboardComponent.GetValueAsBool` _returnvalue_5 "HasTarget")
                    (if (< (`KismetMathLibrary.VSize` (- (`self.K2_GetActorLocation`) (`self.K2_GetActorLocation` (`ActorComponent.GetOwner` Target)))) (`KismetMathLibrary.VSize` (- (`self.K2_GetActorLocation` _returnvalue_2) (`BlackboardComponent.GetValueAsVector` _returnvalue_5 "TargetLocation"))))
                      (if (`/Game/RPGSystem/Blueprints/Utilities/BPL_RPG_Utilities.IsValidTargetAI` (`self.RPGSystem`) Target) :!label _label_2
                        (bind (_outhit _returnvalue_6) (`KismetSystemLibrary.LineTraceSingle` (`self.K2_GetActorLocation` _returnvalue_3) (`self.K2_GetActorLocation` (`ActorComponent.GetOwner` Target)) "TraceTypeQuery5" false (`|MakeArray` _returnvalue_3 :!type "Actor Object Reference")))
                        (if (not _returnvalue_6)
                          (goto _label))))
                    (else
                      (goto _label_2)))))))
          (:`then_1`
            (`PawnSensingComponent.SetSensingInterval` (`self.PawnSensing`) (`KismetMathLibrary.RandomFloatInRange` 0.2 1.5))))))))

(fn `DisableDispatchers`
  (bind _followermaster (`/Game/RPGSystem/Blueprints/BPC_RPGSystem.FollowerMaster` (`self.RPGSystem`)))
  (remove `/Game/RPGSystem/Blueprints/BPC_RPGSystem.OnDamageTaken` (`self.RPGSystem`) (`|CreateDelegate` :!event `OnDamageTaken`))
  (`|ExecutionSequence`
    (:`then_0`
      (if (`|EnumEquality` (cast `/Game/RPGSystem/Blueprints/Enum/Companion/E_FollowerType` (`BlackboardComponent.GetValueAsEnum` (`AIBlueprintHelperLibrary.GetBlackboard` null) "FollowerType")) "NewEnumerator1")
        (`/Engine/EditorBlueprintResources/StandardMacros.IsValid` _followermaster
          (:`Is Valid`
            (remove `/Game/RPGSystem/Blueprints/BPC_RPGSystem.OnMinionMasterNewTarget` _followermaster (`|CreateDelegate` :!event `MasterNewTarget`))))))
    (:`then_1`
      (if (`BlackboardComponent.GetValueAsBool` (`AIBlueprintHelperLibrary.GetBlackboard` null) "IsMaster")
        (remove `/Game/RPGSystem/Blueprints/BPC_RPGSystem.OnMinionNewTarget` (`self.RPGSystem`) (`|CreateDelegate` :!event `MinionNewTarget`))))))

(fn `EnableDispatchers`
  (bind _followermaster (`/Game/RPGSystem/Blueprints/BPC_RPGSystem.FollowerMaster` (`self.RPGSystem`)))
  (add `/Game/RPGSystem/Blueprints/BPC_RPGSystem.OnDamageTaken` (`self.RPGSystem`) (`|CreateDelegate` :!event `OnDamageTaken`))
  (`|ExecutionSequence`
    (:`then_0`
      (if (`|EnumEquality` (cast `/Game/RPGSystem/Blueprints/Enum/Companion/E_FollowerType` (`BlackboardComponent.GetValueAsEnum` (`AIBlueprintHelperLibrary.GetBlackboard` null) "FollowerType")) "NewEnumerator1")
        (`/Engine/EditorBlueprintResources/StandardMacros.IsValid` _followermaster
          (:`Is Valid`
            (add `/Game/RPGSystem/Blueprints/BPC_RPGSystem.OnMinionMasterNewTarget` _followermaster (`|CreateDelegate` :!event `MasterNewTarget`))))))
    (:`then_1`
      (if (`BlackboardComponent.GetValueAsBool` (`AIBlueprintHelperLibrary.GetBlackboard` null) "IsMaster")
        (add `/Game/RPGSystem/Blueprints/BPC_RPGSystem.OnMinionNewTarget` (`self.RPGSystem`) (`|CreateDelegate` :!event `MinionNewTarget`))))))

(fn `UserConstructionScript`)