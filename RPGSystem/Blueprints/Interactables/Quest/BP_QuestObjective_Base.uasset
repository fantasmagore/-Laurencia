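; Base quest objective actor that shows a question-mark marker when its quest is accepted and removes it on completion.
; Construction reads quest type, goal and privacy from the matching task in the quest DataTable.
; On authority, it binds to GameMode dispatchers for quest messages and task variable changes.
; These call empty events for children to override, and any task variable update removes the marker without checking the goal.
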(event `OnQuestAccepted`)

(event `self.ReceiveBeginPlay`
  (`parent.ReceiveBeginPlay`)
  (`self.BindQuestDispatcher`))

(event `OnQuestCompleted`)

(event `OnTaskUpdated`)

(event `self.ReceiveDestroyed`
  (`self.UnbindQuestDispatcher`))

(event `OnQuestStateUpdated`
  (params (Message :type Name) (UniqueID :type Name))
  (switch `name` Message
    (:`Accepted`
      (`self.OnQuestAccepted`)
      (`self.CreateMarker`))
    (:`Completed`
      (`self.OnQuestCompleted`)
      (`self.RemoveMarker`))))

(event `/Game/RPGSystem/Blueprints/Utilities/BPI_RPG_CustomDispatcher.OnCustomDispatcher`
  (params (DispatcherID :type Name) (Message :type Name))
  (`self.OnQuestStateUpdated` Message))

(event `/Game/RPGSystem/Blueprints/Utilities/BPI_RPG_CustomDispatcher.OnCustomDispatcherPrivate`
  (params (DispatcherID :type Name) (Message :type Name) (UniqueID :type String))
  (`self.OnQuestStateUpdated` Message (`KismetStringLibrary.Conv_StringToName` UniqueID)))

(event `/Game/RPGSystem/Blueprints/Utilities/BPI_RPG_CustomDispatcher.OnCustomDispatcherVariable`
  (params (Variable :type Name) (Value :type Integer))
  (`self.OnTaskVariableUpdated` Variable Value))

(event `OnTaskVariableUpdated`
  (params (Variable :type Name) (Value :type Integer))
  (`self.OnTaskUpdated`)
  (`self.RemoveMarker`))

(event `/Game/RPGSystem/Blueprints/Utilities/BPI_RPG_CustomDispatcher.OnCustomDispatcherVariablePrivate`
  (params (Variable :type Name) (Value :type Integer) (UniqueID :type String))
  (`self.OnTaskVariableUpdated` Variable Value))

(fn `BindQuestDispatcher`
  (`/Engine/EditorBlueprintResources/ActorMacros.Switch Has Authority`
    (:`Authority`
      (message `/Game/RPGSystem/Blueprints/Utilities/BPI_RPG_GameMode.BindCustomDispatcher` (`GameplayStatics.GetGameMode`) self (`KismetStringLibrary.Conv_StringToName` (`KismetStringLibrary.Concat_StrStr` "Quest." (`KismetStringLibrary.Conv_NameToString` (`self.QuestID`)))))
      (if (!= (`self.TaskCustomVariable`) "None")
        (message `/Game/RPGSystem/Blueprints/Utilities/BPI_RPG_GameMode.BindCustomDispatcherVariable` (`GameplayStatics.GetGameMode`) self (`self.TaskCustomVariable`) 0 (`self.PrivateTask`))))))

(fn `CreateMarker`
  (bind _returnvalue (`|CreateWidget` "/Game/RPGSystem/Blueprints/UI/Quest/Marker/WBP_QuestMarker_Question.WBP_QuestMarker_Question_C" null (`self.Quest Type`)))
  (`WidgetComponent.SetWidget` (`self.MarkerWidget`) _returnvalue))

(fn `GetTaskInfo`
  (locals (VarQuest_DT :type "DataTable Object Reference"))
  (bind _returnvalue (`|GetDataTableRow` (`local.VarQuest_DT`) (`self.QuestID`))
    (:`then`
      (bind ((`Type_5_50E4B8634F586F3F32BF1CBCC723AFED` _type) (`Tasks_40_0036AE284FC94A23EE666397523E677D` _tasks)) (break `/Game/RPGSystem/Blueprints/Structure/Quest/S_QuestInfo` _returnvalue))
      (for _array_element _tasks
        (bind ((`TaskType_29_A3BE3AB04C577B0E4CADCCAAE0EB7716` _tasktype) (`TrackCustomVariable_42_770EB7C0476297B5449F4BB21506FB82` _trackcustomvariable) (`TrackCustomVariableTag_43_9ABA03A84CB1274FD318D68869B2587D` _trackcustomvariabletag) (`CustomVariableValueGoal_56_A6AEF61345F84815D7B8A38E8D03FC56` _customvariablevaluegoal) (`PrivateVariable_59_FC6249024CCE38155CDBE5A0328604E0` _privatevariable)) (break `/Game/RPGSystem/Blueprints/Structure/Quest/S_Quest_TaskEntry` _array_element))
        (if (or (== _trackcustomvariable (`self.TaskCustomVariable`)) (== _trackcustomvariabletag (`self.TaskCustomVariableTag`)))
          (set `self.Quest Type` _type)
          (set `self.TaskGoal` _customvariablevaluegoal)
          (set `self.PrivateTask` _privatevariable)
          (return))))))

(fn `RemoveMarker`
  (bind _returnvalue (`WidgetComponent.GetWidget` (`self.MarkerWidget`)))
  (`/Engine/EditorBlueprintResources/StandardMacros.IsValid` _returnvalue
    (:`Is Valid`
      (`Widget.RemoveFromParent` _returnvalue)
      (`WidgetComponent.SetWidget` (`self.MarkerWidget`) null))))

(fn `UnbindQuestDispatcher`
  (`/Engine/EditorBlueprintResources/ActorMacros.Switch Has Authority`
    (:`Authority`
      (message `/Game/RPGSystem/Blueprints/Utilities/BPI_RPG_GameMode.UnbindCustomDispatcher` (`GameplayStatics.GetGameMode`) self (`KismetStringLibrary.Conv_StringToName` (`KismetStringLibrary.Concat_StrStr` "Quest." (`KismetStringLibrary.Conv_NameToString` (`self.QuestID`)))))
      (if (!= (`self.TaskCustomVariable`) "None")
        (message `/Game/RPGSystem/Blueprints/Utilities/BPI_RPG_GameMode.UnbindCustomDispatcherVariable` (`GameplayStatics.GetGameMode`) self (`KismetStringLibrary.Conv_StringToName` (`KismetStringLibrary.Concat_StrStr` "Quest." (`KismetStringLibrary.Conv_NameToString` (`self.QuestID`)))) 0 (`self.PrivateTask`))))))

(fn `UserConstructionScript`
  (`parent.UserConstructionScript`)
  (`self.GetTaskInfo`))