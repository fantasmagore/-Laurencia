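; Example shop NPC interactable for the RPG system that highlights its skeletal mesh through custom depth when selected.
; Interact forwards to the parent implementation, which handles the actual shop behavior.
; A disconnected, never-executed example shows how a server-side interaction could send a custom variable message to the game instance to update a quest task variable for that player.
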(event `/Game/RPGSystem/Blueprints/Utilities/BPI_RPG_Interaction.SelectInteractable`
  (params (Selected :type Boolean))
  ;[1 1 1] Outline
  (`PrimitiveComponent.SetRenderCustomDepth` (`self.SkeletalMesh`) Selected))

(event `/Game/RPGSystem/Blueprints/Utilities/BPI_RPG_Interaction.Interact`
  (params (Player :type "/Game/RPGSystem/Blueprints/BPC_RPGSystem Object Reference") (Command :type String))
  (`parent.Interact` Player Command))

(fn `UserConstructionScript`
  (`parent.UserConstructionScript`))