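; Base Blueprint for shopkeeper NPCs, which lets a player open or close a shop by interacting with it.
; Interact toggles the shop: it closes the player's current shop if one is valid, otherwise it opens this NPC's BPCShop component.
; Tooltip-triggered interactions toggle only when the interact info's action is the first enum entry, while other commands toggle directly.
; GetShopComponent exposes the shop component to callers.
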(event `/Game/RPGSystem/Blueprints/Utilities/BPI_RPG_Interaction.Interact`
  (params (Player :type "/Game/RPGSystem/Blueprints/BPC_RPGSystem Object Reference") (Command :type String))
  ;[1 1 1] Interact
  (if (`KismetStringLibrary.EqualEqual_StrStr` Command "FromTooltip")
    (bind (_success _type _action) (`self.GetInteractInfo` Player))
    (if (`|EnumEquality` _action "NewEnumerator0")
      (`/Engine/EditorBlueprintResources/StandardMacros.IsValid` (`/Game/RPGSystem/Blueprints/BPC_RPGSystem.CurrentShop` Player) :!label _label
        (:`Is Valid`
          (`/Game/RPGSystem/Blueprints/BPC_RPGSystem.CloseShop` Player))
        (:`Is Not Valid`
          (`/Game/RPGSystem/Blueprints/BPC_RPGSystem.OpenShop` Player (`self.BPC_Shop`)))))
    (else
      (goto _label))))

(fn `GetShopComponent`
  (returns (Success :type Boolean) (Component :type "/Game/RPGSystem/Blueprints/BPC_Shop Object Reference"))
  (return true (`self.BPC_Shop`)))

(fn `UserConstructionScript`)