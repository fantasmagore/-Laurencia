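; Base waypoint interactable for the RPG system that becomes a player's last waypoint when a non-AI player overlaps it.
; Overlap sends a server interact and predicts it locally, spawning a particle effect when the waypoint is new to that player.
; The construction script generates an optionally centered, rotated grid of PlayerStarts, tagging them and assigned SpawnPoints with WaypointID.
; A data table row supplies the Waypoint or Checkpoint tooltip.
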(event `self.ReceiveBeginPlay`
  (`parent.ReceiveBeginPlay`)
  (bind _returnvalue (`|GetDataTableRow` (`self.Waypoint_DT`) (`self.WaypointID`))
    (:`then`
      (bind ((`Name_2_1DA64F4D4237C567AAA921B51BA5EF7B` _name) (`Checkpoint_32_94D77DF745A3046EC886F49E14006599` _checkpoint)) (break `/Game/RPGSystem/Blueprints/Structure/Waypoint/S_WaypointData` _returnvalue))
      (set `self.WorldTooltipText` (`|FormatText` "{0} {1}" _name (select `bool` _checkpoint :`false` "Waypoint" :`true` "Checkpoint" :!type "Text"))))))

(event `/Game/RPGSystem/Blueprints/Utilities/BPI_RPG_Interaction.Interact`
  (params (Player :type "/Game/RPGSystem/Blueprints/BPC_RPGSystem Object Reference") (Command :type String))
  (`parent.Interact` Player Command)
  (`/Engine/EditorBlueprintResources/StandardMacros.IsValid` Player
    (:`Is Valid`
      (if (!= (`/Game/RPGSystem/Blueprints/BPC_RPGSystem.GetLastWaypoint` Player) (`self.WaypointID`))
        (`/Game/RPGSystem/Blueprints/BPC_RPGSystem.SetLastWaypoint` Player (`self.WaypointID`))
        (`GameplayStatics.SpawnEmitterAttached` "/Game/RPGSystem/Particles/P_Greystone_Novaborn_HToKill_Resurrect.P_Greystone_Novaborn_HToKill_Resurrect" (`self.DefaultSceneRoot`) "None" (0.0 0.0 50.0) (struct) (0.25 0.25 0.25))))))

(event `self.TriggerCollision.OnComponentBeginOverlap`
  (params (OverlappedComponent :type "PrimitiveComponent Object Reference") (OtherActor :type "Actor Object Reference") (OtherComp :type "PrimitiveComponent Object Reference") (OtherBodyIndex :type Integer) (bFromSweep :type Boolean) (SweepResult :type "HitResult Structure (by ref)"))
  (bind (_success _reference) (message `/Game/RPGSystem/Blueprints/Utilities/BPI_RPG_PlayerCharacter.GetRPGSystem` OtherActor))
  (if _success
    (if (not (`/Game/RPGSystem/Blueprints/BPC_RPGSystem.PlayerAI` _reference))
      (`/Game/RPGSystem/Blueprints/BPC_RPGSystem.InteractServer` _reference self "")
      (`self.Interact` _reference) ; Client Particle prediction
    )))

(fn `GeneratePointsBox`
  (locals (VarForwardDistance :type "Vector Structure") (VarRowIndex :type Integer) (VarColumnIndex :type Integer) (VarOffset :type "Vector2D Structure") (VarMiddleColumn :type "Float (double-precision)") (VarEven :type Boolean))
  (bind _startdistanceup (`self.StartDistanceUp`))
  (bind _varcolumnindex (`local.VarColumnIndex`))
  (bind (_x _y) (`KismetMathLibrary.BreakVector2D` (`local.VarOffset`)))
  (bind _returnvalue (+ (`self.StartDistance`) _y))
  (bind _returnvalue_2 (* (`self.ColumnSpacing`) (`KismetMathLibrary.Round` (/ (`KismetMathLibrary.Conv_IntToDouble` _varcolumnindex) 2.0))))
  (`self.K2_DestroyActor` (`self.AutoSpawnedPoints`))
  (set `local.VarEven` (== (mod (`self.NumColumns`) 2) 0))
  (for _index (range (`self.Count`))
    (set `local.VarColumnIndex` (mod _index (`self.NumColumns`)))
    (set `local.VarRowIndex` (/ _index (`self.NumColumns`)))
    (set `local.VarOffset` (`KismetMathLibrary.MakeVector2D` (`KismetMathLibrary.SelectFloat` (+ (`KismetMathLibrary.SelectFloat` (* _returnvalue_2 -1.0) _returnvalue_2 (== (mod (- _varcolumnindex 1) 2) 0)) (`KismetMathLibrary.SelectFloat` (/ (`self.ColumnSpacing`) 2.0) 0.0 (`local.VarEven`))) (* (`local.VarColumnIndex`) (`self.ColumnSpacing`)) (`self.Centered`)) (* (`local.VarRowIndex`) (`self.RowSpacing`))))
    (bind _returnvalue_3 (`AddComponent|NODE_AddChildActorComponent-2` :`bManualAttachment` true :`RelativeTransform` (`KismetMathLibrary.MakeTransform` (`KismetMathLibrary.MakeVector` _returnvalue _x _startdistanceup) (`KismetMathLibrary.MakeRotator` 0.0 0.0 (`self.RotationOffset`)))))
    (`SceneComponent.K2_SetRelativeLocation` _returnvalue_3 (+ (`KismetMathLibrary.GreaterGreater_VectorRotator` (`KismetMathLibrary.MakeVector` _returnvalue _x _startdistanceup) (`self.K2_GetActorRotation`)) (`self.K2_GetActorLocation`)) false true)
    (bind _asplayer_start (cast `PlayerStart` (`ChildActorComponent.ChildActor` _returnvalue_3)))
    (`KismetArrayLibrary.Array_Add` (`self.AutoSpawnedPoints`) _asplayer_start)))

(fn `GetWorldTooltipInfo`
  (params (HitComp :type "PrimitiveComponent Object Reference"))
  (returns (Success :type Boolean) (Interactable :type Boolean) (Text :type Text) (Color :type "LinearColor Structure") (Offset :type "Vector Structure"))
  (locals (VarWaypointDT :type "DataTable Object Reference" :default "/Script/Engine.CompositeDataTable'/Game/RPGSystem/Blueprints/Database/Composite/CDT_Waypoint.CDT_Waypoint'"))
  (return true false (`self.WorldTooltipText`) (struct) (0.0 0.0 150.0)))

(fn `ResetLastIndex`
  (set `self.LastUsedSpawnIndex` -1))

(fn `UserConstructionScript`
  (`self.GeneratePointsBox`)
  (bind _arrayelement (`/Game/RPGSystem/Blueprints/Utilities/BML_RPG_Utilities.ForeachLoopByRef` (`self.AutoSpawnedPoints`))
    (:`Body`
      (set `PlayerStart.PlayerStartTag` (`self.WaypointID`) _arrayelement))
    (:`Complete`
      (bind _arrayelement_2 (`/Game/RPGSystem/Blueprints/Utilities/BML_RPG_Utilities.ForeachLoopByRef` (`self.SpawnPoints`))
        (:`Body`
          (set `PlayerStart.PlayerStartTag` (`self.WaypointID`) _arrayelement_2))))))