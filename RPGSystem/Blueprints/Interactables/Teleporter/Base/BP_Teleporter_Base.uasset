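; Base interactable teleporter that sends an interacting player to the waypoint named by its Waypoint ID.
; On BeginPlay it looks up that ID in the waypoint data table and sets the world tooltip to the row's name, or to an invalid-ID message.
; Interact runs the parent logic, then calls TeleportToWaypoint only on the server and only for players not flagged as AI.
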(event `self.ReceiveBeginPlay`
  (`parent.ReceiveBeginPlay`)
  (bind _returnvalue (`|GetDataTableRow` (`self.Waypoint_DT`) (`self.Waypoint`))
    (:`then`
      (set `self.WorldTooltipText` (`.Name_2_1DA64F4D4237C567AAA921B51BA5EF7B` (break `/Game/RPGSystem/Blueprints/Structure/Waypoint/S_WaypointData` _returnvalue))))
    (:`RowNotFound`
      (set `self.WorldTooltipText` "Invalid WaypointID"))))

(event `/Game/RPGSystem/Blueprints/Utilities/BPI_RPG_Interaction.Interact`
  (params (Player :type "/Game/RPGSystem/Blueprints/BPC_RPGSystem Object Reference") (Command :type String))
  (`parent.Interact` Player Command)
  (`/Engine/EditorBlueprintResources/ActorMacros.Switch Has Authority`
    (:`Authority`
      (if (not (`/Game/RPGSystem/Blueprints/BPC_RPGSystem.PlayerAI` Player))
        (`/Game/RPGSystem/Blueprints/Utilities/BPL_RPG_Utilities.Teleport To Waypoint` Player (`self.Waypoint`))))))

(fn `UserConstructionScript`)