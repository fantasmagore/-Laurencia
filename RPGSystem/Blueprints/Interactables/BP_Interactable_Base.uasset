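; Base actor for RPG interactables, supplying interaction checks, move and look-at targets, and screen and world tooltips.
; GetInteractInfo returns MoveTo, RotateTo or Interact from the player's range and facing angle.
; The move goal is either a rotated fixed offset or a bounds-based point on the player's side.
; On authority, Interact increments or creates global and per-player custom variables, named or tag-based, through GameInstance messages.
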(event `/Game/RPGSystem/Blueprints/Utilities/BPI_RPG_Interaction.Interact`
  (params (Player :type "/Game/RPGSystem/Blueprints/BPC_RPGSystem Object Reference") (Command :type String))
  ;[1 1 1] Add CustomVariables to the Player
  (`/Engine/EditorBlueprintResources/ActorMacros.Switch Has Authority`
    (:`Authority`
      (`self.AddCustomVariablesToPlayer` (`/Game/RPGSystem/Blueprints/BPC_RPGSystem.GetUniqueID` Player)))))

(fn `AddCustomVariablesToPlayer`
  (params (UniqueID :type String))
  (bind (_global _private) (`self.GetCustomVariables`))
  (for _array_element (`.List_3_898F375A44F28AA8331C7991FD607384` (break `/Game/RPGSystem/Blueprints/Structure/Misc/S_ArrayOf_FName` _global))
    (bind _success (message `/Game/RPGSystem/Blueprints/Utilities/BPI_RPG_CustomVariable.GetCustomVariableValue` (`GameplayStatics.GetGameInstance`) _array_element ""))
    (if _success
      (message `/Game/RPGSystem/Blueprints/Utilities/BPI_RPG_CustomVariable.SetCustomVariableValue` (`GameplayStatics.GetGameInstance`) _array_element 1 true "")
      (else
        (message `/Game/RPGSystem/Blueprints/Utilities/BPI_RPG_CustomVariable.AddCustomVariable` (`GameplayStatics.GetGameInstance`) _array_element 1 ""))))
  (for _array_element_2 (`.List_3_898F375A44F28AA8331C7991FD607384` (break `/Game/RPGSystem/Blueprints/Structure/Misc/S_ArrayOf_FName` _private))
    (bind _success_2 (message `/Game/RPGSystem/Blueprints/Utilities/BPI_RPG_CustomVariable.GetCustomVariableValue` (`GameplayStatics.GetGameInstance`) _array_element_2 (`local.UniqueID`)))
    (if _success_2
      (message `/Game/RPGSystem/Blueprints/Utilities/BPI_RPG_CustomVariable.SetCustomVariableValue` (`GameplayStatics.GetGameInstance`) _array_element_2 1 true (`local.UniqueID`))
      (else
        (message `/Game/RPGSystem/Blueprints/Utilities/BPI_RPG_CustomVariable.AddCustomVariable` (`GameplayStatics.GetGameInstance`) _array_element_2 1 (`local.UniqueID`))))))

(fn `GetCustomVariables`
  (returns (Global :type "/Game/RPGSystem/Blueprints/Structure/Misc/S_ArrayOf_FName Structure") (Private :type "/Game/RPGSystem/Blueprints/Structure/Misc/S_ArrayOf_FName Structure"))
  (locals (VarCustomVariables :type "Array of Name") (VarCustomVariablesPrivate :type "Array of Name"))
  (bind (_global _private _globaltag _privatetag) (break `/Game/RPGSystem/Blueprints/Structure/CustomVariable/S_CustomVariable_OnExpose` (`self.CustomVariables`)))
  (set `local.VarCustomVariables` _global)
  (set `local.VarCustomVariablesPrivate` _private)
  (for _array_element _globaltag
    (`KismetArrayLibrary.Array_Add` (`local.VarCustomVariables`) (`BlueprintGameplayTagLibrary.GetTagName` _array_element)))
  (for _array_element_2 _privatetag
    (`KismetArrayLibrary.Array_Add` (`local.VarCustomVariablesPrivate`) (`BlueprintGameplayTagLibrary.GetTagName` _array_element_2)))
  (return (make `/Game/RPGSystem/Blueprints/Structure/Misc/S_ArrayOf_FName` (`local.VarCustomVariables`)) (make `/Game/RPGSystem/Blueprints/Structure/Misc/S_ArrayOf_FName` (`local.VarCustomVariablesPrivate`))))

(fn `GetInteractableComponents`
  (returns (Components :type "Array of PrimitiveComponent Object Reference"))
  (return))

(fn `GetInteractInfo`
  (params (Player :type "/Game/RPGSystem/Blueprints/BPC_RPGSystem Object Reference"))
  (returns (Success :type Boolean) (Type :type "/Game/RPGSystem/Blueprints/Enum/Interact/E_InteractType Enum") (Action :type "/Game/RPGSystem/Blueprints/Enum/Interact/E_InteractAction Enum"))
  (locals (VarRadius :type "Float (double-precision)" :default 0.0) (VarHeight :type "Float (double-precision)" :default 0.0))
  (bind _returnvalue (`ActorComponent.GetOwner` (`local.Player`)))
  (bind _returnvalue_2 (`ActorComponent.GetOwner` (`local.Player`)))
  (bind _returnvalue_3 (`self.K2_GetActorLocation` _returnvalue_2))
  (bind _range (message `/Game/RPGSystem/Blueprints/Utilities/BPI_RPG_PlayerController.GetInteractionRange` (`self.GetInstigatorController` _returnvalue)))
  (bind (_radius _halfheight) (message `/Game/RPGSystem/Blueprints/Utilities/BPI_RPG_PlayerCharacter.GetMeshRadius` _returnvalue))
  (bind _worldlocation (`self.GetMoveToEndDestination` (`local.Player`)))
  (if (<= (`/Game/RPGSystem/Blueprints/Utilities/BPL_RPG_Utilities.GetDistanceExt` _returnvalue_3 _worldlocation _radius (* _halfheight 2.0)) _range)
    (bind _return (`self.GetLookAtLocation`))
    (if (`/Game/RPGSystem/Blueprints/Utilities/BPL_RPG_Utilities.IsTargetInAngle` _return _returnvalue_3 (`self.GetActorForwardVector` _returnvalue_2) (`self.LookAt_MinAngle`))
      (return true (`self.Type`) "NewEnumerator0")
      (else
        (return true (`self.Type`) "NewEnumerator5")))
    (else
      (return true (`self.Type`) "NewEnumerator1"))))

(fn `GetLookAtLocation`
  (returns (Return :type "Vector Structure"))
  (return (`SceneComponent.K2_GetComponentLocation` (`self.DefaultSceneRoot`))))

(fn `GetMoveToEndDestination`
  (params (Player :type "/Game/RPGSystem/Blueprints/BPC_RPGSystem Object Reference"))
  (returns (WorldLocation :type "Vector Structure"))
  (bind (_origin _boxextent) (`self.GetActorBounds` true))
  (if (`self.UseMoveGoal`)
    (return (+ (`self.K2_GetActorLocation`) (`KismetMathLibrary.GreaterGreater_VectorRotator` (`self.MoveGoal`) (`self.K2_GetActorRotation`))))
    (else
      (return (+ (- _origin (`KismetMathLibrary.MakeVector` 0.0 0.0 (.z _boxextent))) (* (`KismetMathLibrary.GetForwardVector` (`KismetMathLibrary.MakeRotator` 0.0 0.0 (.yaw (`KismetMathLibrary.FindLookAtRotation` (`self.K2_GetActorLocation`) (`self.K2_GetActorLocation` (`ActorComponent.GetOwner` (`local.Player`))))))) (+ (`KismetMathLibrary.VSize` _boxextent) (`self.MoveGoal_Offset`))))))))

(fn `GetScreenTooltipInfo`
  (params (Player :type "/Game/RPGSystem/Blueprints/BPC_RPGSystem Object Reference"))
  (returns (Success :type Boolean) (Text :type Text) (Color :type "LinearColor Structure"))
  (bind (_success _type _action) (`self.GetInteractInfo` Player)) ; Checking distance
  (return (`self.ShowScreenTooltip`) (select `/Game/RPGSystem/Blueprints/Enum/Interact/E_InteractAction` _action :`NewEnumerator0` (`|FormatText` (`self.KeypromptFormat`) (`self.InteractScreenText`) (`KismetInputLibrary.Key_GetDisplayName` (`|GetArrayItem` (`EnhancedInputSubsystemInterface.QueryKeysMappedToAction` (subsystem `EnhancedInputWorldSubsystem`) (`self.InputAction`))))) :`NewEnumerator1` "RPG_InteractFarAway") (struct :`R` 1.0 :`G` 1.0 :`B` 1.0 :`A` 1.0)))

(fn `GetTeamID`
  (returns (Return :type String))
  (return ""))

(fn `GetWorldTooltipInfo`
  (params (HitComp :type "PrimitiveComponent Object Reference"))
  (returns (Success :type Boolean) (Interactable :type Boolean) (Text :type Text) (Color :type "LinearColor Structure") (Offset :type "Vector Structure"))
  (return (`self.ShowWorldTooltip`) (`self.InteractableTooltip`) (`self.WorldTooltipText`) (struct :`R` 1.0 :`G` 1.0 :`B` 1.0 :`A` 1.0) (`self.WorldTooltipOffset`)))

(fn `IsDamageable`
  (params (TeamID :type String))
  (returns (Return :type Boolean))
  (return false))

(fn `UserConstructionScript`)