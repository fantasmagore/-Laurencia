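; Base interactable treasure that opens once on server-side interaction and drops loot, with an outline highlight while selected.
; Tooltip interactions are validated through GetInteractInfo when a tooltip exists; other commands open it directly.
; Opening records custom variables on the player, then after a short delay feeds player level, drop and gold bonuses to BPCDropSystem.
; The replicated Open flag's OnRep plays the mesh animation and clears the outline.
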(event `/Game/RPGSystem/Blueprints/Utilities/BPI_RPG_Interaction.SelectInteractable`
  (params (Selected :type Boolean))
  ;[1 1 1] Outline
  (`PrimitiveComponent.SetRenderCustomDepth` (`self.SkeletalMesh`) Selected))

(event `/Game/RPGSystem/Blueprints/Utilities/BPI_RPG_Interaction.Interact`
  (params (Player :type "/Game/RPGSystem/Blueprints/BPC_RPGSystem Object Reference") (Command :type String))
  ;[1 1 1] Interact
  (`/Engine/EditorBlueprintResources/ActorMacros.Switch Has Authority`
    (:`Authority`
      (if (`self.Open`)
        _
        (elif (`KismetStringLibrary.EqualEqual_StrStr` Command "FromTooltip")
          (if (`self.InteractableTooltip`)
            (bind (_success _type _action) (`self.GetInteractInfo` Player))
            (if _success
              (switch `/Game/RPGSystem/Blueprints/Enum/Interact/E_InteractAction` _action
                (:`NewEnumerator0`
                  (set `self.Open` true :!label _label)
                  (bind _output_get (set `self.Player` Player))
                  (`self.AddCustomVariablesToPlayer` (`/Game/RPGSystem/Blueprints/BPC_RPGSystem.GetUniqueID` _output_get))
                  (`KismetSystemLibrary.Delay` 0.6)
                  (`self.StartDrop`)
                  (`self.OnOpenTreasure`))))
            (else
              (goto _label)))
          (else
            (goto _label)))))))

(event `StartDrop`
  (bind _player (`self.Player`))
  (bind (_returnvalue_location _returnvalue_rotation) (`KismetMathLibrary.BreakTransform` (`SceneComponent.K2_GetComponentToWorld` (`self.DropPoint`))))
  ;[1 1 1] Start Drop
  (`/Game/RPGSystem/Blueprints/BPC_DropSystem.StartDrop` (`self.BPC_DropSystem`) (`/Game/RPGSystem/Blueprints/BPC_RPGSystem.GetBaseLevel` _player) (`.Percent` (`/Game/RPGSystem/Blueprints/BPC_RPGSystem.GetStatBonus` _player "NewEnumerator65")) (`.Percent` (`/Game/RPGSystem/Blueprints/BPC_RPGSystem.GetStatBonus` _player "NewEnumerator64")) _returnvalue_location _returnvalue_rotation))

(fn `OnRep_Open`
  (`SkeletalMeshComponent.Play` (`self.SkeletalMesh`) false)
  (`PrimitiveComponent.SetRenderCustomDepth` (`self.SkeletalMesh`) false))

(fn `UserConstructionScript`
  (locals (NewLocalVar_0 :type "Float (double-precision)" :default 1.0))
  (`parent.UserConstructionScript`))