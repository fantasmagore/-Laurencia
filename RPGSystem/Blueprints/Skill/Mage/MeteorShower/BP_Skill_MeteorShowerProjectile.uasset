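; Single meteor projectile for the Mage Meteor Shower skill, landing at a randomly scattered point around its spawn location.
; On skill start it jumps to an elevated offset, traces toward the target for the impact point, and spawns a client particle spawner.
; A timeline lerps it down, then plays camera shake and impact effects.
; The parent skill logic fires only on impact, followed by delayed trail shutdown and destruction.
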(event `self.ReceiveBeginPlay`
  (bind _returnvalue (+ (`self.K2_GetActorLocation`) (`KismetMathLibrary.MakeVector` (`KismetMathLibrary.RandomFloatInRange` -250.0 250.0) (`KismetMathLibrary.RandomFloatInRange` -250.0 250.0))))
  (`self.K2_SetActorLocation` _returnvalue false true)
  (set `self.StartLocation` _returnvalue)
  (setmembers `/Game/RPGSystem/Blueprints/Structure/Skill/S_Skill` :`StructRef` (`self.SkillInfo`))
  (`parent.ReceiveBeginPlay`))

(event `EndTrail`
  (bind _particlesystem (`self.ParticleSystem`))
  (`KismetSystemLibrary.Delay` 5.0)
  (`/Engine/EditorBlueprintResources/StandardMacros.IsValid` _particlesystem
    (:`Is Valid`
      (`ParticleSystemComponent.EndTrails` _particlesystem))
    (:`Is Not Valid`
      _))
  (`KismetSystemLibrary.Delay` 1.0)
  (`self.K2_DestroyActor`))

(event `StartMeteor`
  (`parent.SkillStart`)
  (`self.EndTrail`))

(event `self.SkillStart`
  (bind _rangeindicator (`self.RangeIndicator`))
  (`self.K2_SetActorLocation` (+ (`self.K2_GetActorLocation`) (`KismetMathLibrary.MakeVector` (`KismetMathLibrary.RandomFloatInRange` -700.0 -1200.0) (`KismetMathLibrary.RandomFloatInRange` -700.0 -1200.0) 1000.0)) false true)
  (bind _outhit (`KismetSystemLibrary.LineTraceSingle` :`Start` (`self.K2_GetActorLocation`) :`End` (`self.StartLocation`) :`TraceChannel` "TraceTypeQuery2" :`TraceColor` (struct :`G` 0.313568 :`B` 1.0 :`A` 1.0)))
  (bind (_bblockinghit _binitialoverlap _time _distance _location) (`GameplayStatics.BreakHitResult` _outhit))
  (bind _returnvalue (`KismetMathLibrary.SelectVector` _location (`self.StartLocation`) _bblockinghit))
  (set `self.EndLocation` _returnvalue)
  (set `self.StartLocation` (`self.K2_GetActorLocation`))
  (`/Engine/EditorBlueprintResources/StandardMacros.IsValid` _rangeindicator
    (:`Is Valid`
      (`SceneComponent.K2_SetWorldLocation` _rangeindicator _returnvalue false true))
    (:`Is Not Valid`
      _))
  (`self.SpawnClientParticle` (`self.StartLocation`) (`self.EndLocation`))
  (bind (_direction _newtrack_0) (`Timeline|BoltMovement` :!via `PlayFromStart`)
    (:`Update`
      (`self.K2_SetActorLocation` (`KismetMathLibrary.VLerp` (`self.StartLocation`) (`self.EndLocation`) _newtrack_0) false true))
    (:`Finished`
      (`GameplayStatics.PlayWorldCameraShake` "/Game/RPGSystem/Blueprints/Camera/Shakes/CS_ExampleShake.CS_ExampleShake_C" (`self.K2_GetActorLocation`) 0.0 2500.0 0.05)
      (`GameplayStatics.SpawnEmitterAtLocation` "/Game/RPGSystem/Particles/P_MeteorImpact.P_MeteorImpact" (`self.K2_GetActorLocation`))
      (`self.StartMeteor`))))

(event `SpawnClientParticle`
  (params (StartLocation :type "Vector Structure") (EndLocation :type "Vector Structure"))
  (`|SpawnActorFromClass` "/Game/RPGSystem/Blueprints/Skill/Mage/MeteorShower/BP_Meteor_ClientSpawner.BP_Meteor_ClientSpawner_C" (`self.GetTransform`) "AlwaysSpawn" "OverrideRootScale" null StartLocation EndLocation null))

(fn `UserConstructionScript`
  (`parent.UserConstructionScript`))