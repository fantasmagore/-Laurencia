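; Short-lived relay actor for the Mage Meteor Shower skill that spawns the client-only meteor projectile.
; On BeginPlay the server passes the start and end locations to SpawnClientParticle, then destroys the actor.
; That event acts only off the server, spawning BP_Skill_MeteorShowerProjectile_Client at the actor's transform with both locations.
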(event `self.ReceiveBeginPlay`
  (if (`KismetSystemLibrary.IsServer`)
    (`self.SpawnClientParticle` (`self.StartLocation`) (`self.EndLocation`))
    (`self.K2_DestroyActor`)))

(event `SpawnClientParticle`
  (params (StartLocation :type "Vector Structure") (EndLocation :type "Vector Structure"))
  (if (not (`KismetSystemLibrary.IsServer`))
    (`|SpawnActorFromClass` "/Game/RPGSystem/Blueprints/Skill/Mage/MeteorShower/BP_Skill_MeteorShowerProjectile_Client.BP_Skill_MeteorShowerProjectile_Client_C" (`self.GetTransform`) "AlwaysSpawn" "OverrideRootScale" null StartLocation EndLocation null 0.0 true null null)))

(fn `UserConstructionScript`)