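; Windstorm skill for the Mage, built on a parent skill class that it extends at skill start.
; On start it caches the configured damage as a maximum and scales the actor to match the trace's sphere radius or box length.
; When the async attack starts, it plays a world camera shake at its location and rerolls damage just below that maximum.
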(event `self.SkillStart`
  (bind ((`Damage_356_051999E94AC01F21023A41B864B49BC7` _damage) (`AsyncAttack_Settings_541_5C9CB04444CB3991BAFDDF8D24D390D2` _asyncattack_settings) (`MaxHitTargets_540_0F374CA64BA9FC88F84E1F9C9A12E389` _maxhittargets) (`Trace_Settings_517_9BFE8A074B33E463AEBCF88884F007C0` _trace_settings)) (break `/Game/RPGSystem/Blueprints/Structure/Skill/S_Skill` (`self.SkillInfo`)))
  (bind (_tracetype _addattackrangetotrace _attackrangeoverwriteai _sphere_settings _box_settings) (break `/Game/RPGSystem/Blueprints/Structure/Skill/S_Skill_TraceData` _trace_settings))
  (set `self.MaxDamage` _damage)
  (`self.SetActorScale3D` (`KismetMathLibrary.Conv_DoubleToVector` (* (/ (select `/Game/RPGSystem/Blueprints/Enum/Skill/E_SkillTraceType` _tracetype :`NewEnumerator0` (`.Radius_19_6BDBC5774B346A254DE606BFD88AD5E7` (break `/Game/RPGSystem/Blueprints/Structure/Skill/S_SkillSphereTraceSettings` _sphere_settings)) :`NewEnumerator1` (`.Length_5_6BDBC5774B346A254DE606BFD88AD5E7` (break `/Game/RPGSystem/Blueprints/Structure/Skill/S_SkillBoxTraceSettings` _box_settings)) :!type "Float (double-precision)") 200.0) 0.55)))
  (`parent.SkillStart`))

(event `self.OnAsyncAttackStarted`
  (bind _maxdamage (`self.MaxDamage`))
  ;[1 1 1] Comment
  (`GameplayStatics.PlayWorldCameraShake` "/Game/RPGSystem/Blueprints/Camera/Shakes/CS_ExampleShake.CS_ExampleShake_C" (`self.K2_GetActorLocation`) 0.0 2500.0 0.05)
  (setmembers `/Game/RPGSystem/Blueprints/Structure/Skill/S_Skill` :`StructRef` (`self.SkillInfo`) :`Damage` (`KismetMathLibrary.RandomFloatInRange` (* _maxdamage 0.98) _maxdamage)))

(fn `UserConstructionScript`
  (`parent.UserConstructionScript`))