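; Mage bolt skill actor that spawns at the caster's left hand and launches characters it hits.
; On BeginPlay it teleports just ahead of the owner's Hand_l socket along its forward vector, then runs the parent logic.
; On hit, it launches a Character target opposite the bolt-to-target direction, pulling it toward the bolt, overriding horizontal velocity only.
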(event `self.ReceiveBeginPlay`
  (bind (_success _component) (message `/Game/RPGSystem/Blueprints/Utilities/BPI_RPG_PlayerCharacter.Get Skeletal Mesh` (`ActorComponent.GetOwner` (`self.SkillOwner`))))
  (`self.K2_SetActorLocation` (+ (`SceneComponent.GetSocketLocation` _component "Hand_l") (* (`self.GetActorForwardVector`) 55.0)) false true)
  (`parent.ReceiveBeginPlay`))

(event `self.OnHit`
  (params (Target :type "/Game/RPGSystem/Blueprints/BPC_RPGSystem Object Reference"))
  (bind _returnvalue (`ActorComponent.GetOwner` Target))
  (bind _ascharacter (cast `Character` _returnvalue))
  (`Character.LaunchCharacter` _ascharacter (* (`KismetMathLibrary.GetForwardVector` (`KismetMathLibrary.FindLookAtRotation` (`self.K2_GetActorLocation`) (`self.K2_GetActorLocation` _returnvalue))) -500.0) true false))

(fn `UserConstructionScript`
  (`parent.UserConstructionScript`))