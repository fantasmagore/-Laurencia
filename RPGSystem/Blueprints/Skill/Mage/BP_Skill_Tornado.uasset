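; BP_Skill_Tornado is a Mage skill that creates a damaging vortex which pulls valid targets toward its center.
; On start it spawns an attached whirl particle timed from the multi-hit settings, starts skill damage and sizes its Sphere from the trace settings.
; Every tick it launches overlapping target characters inward, scaled by distance, until they are near the center allowing for mesh radius.
; After each hit it slightly randomizes damage below the initial maximum.
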(event `self.SkillStart`
  (bind ((`AttackType_444_ACFCC5534FFDE6843948798661995027` _attacktype) (`RangeType_433_40B0C27A44C55567BD541FA9DFEFE11C` _rangetype) (`DamageType_447_EE2BF99A40D6A48A6A413B83DA01433D` _damagetype) (`HealthTypeConsume_427_B53CF6F740B4AEF8B7A0C68B86A53898` _healthtypeconsume) (`DamageTo_430_DF73400C4C328B774F753083EA39EB5E` _damageto) (`Damage_356_051999E94AC01F21023A41B864B49BC7` _damage) (`DamagePercent_357_50D9E6784A2908832B46C2B0A83D478C` _damagepercent) (`FixedDamage_358_212AAC024782C20480D70FA876ABC285` _fixeddamage) (`MultiHitCount_136_4FE79D72405666B66DD53AA3CA1C52B4` _multihitcount) (`MultiHitDelay_139_89305FE94279297B9E1BB79D4A8A1A34` _multihitdelay) (`CritBonus_448_3B57C4364598C5F583267DB033D55A4F` _critbonus) (`SkillExecutionType_395_2316A0914386027A9506BA993F280FFB` _skillexecutiontype) (`Projectile_Settings_509_A79BB4BB40B6ED6488BE1996BE5FFA52` _projectile_settings) (`Targeting_Settings_511_7CC7E835443906B956308ABA2E8C8EF7` _targeting_settings) (`Spawn_Settings_513_553A9A9A4228718D2171CC868CBDD6C6` _spawn_settings) (`RotateTo_Settings_515_ED859EE64B73CE23997E01B3893AEA09` _rotateto_settings) (`AsyncAttack_Settings_541_5C9CB04444CB3991BAFDDF8D24D390D2` _asyncattack_settings) (`MaxHitTargets_540_0F374CA64BA9FC88F84E1F9C9A12E389` _maxhittargets) (`Trace_Settings_517_9BFE8A074B33E463AEBCF88884F007C0` _trace_settings) (`ShowSkillIndicator_482_774D95804CA28F9C129BCDBAE9E629A8` _showskillindicator) (`Ragdoll_Force_546_D5103DEE45AF6CE66D58DFBCAB5BFA12` _ragdoll_force) (`Ragdoll_Force_Origin_Offset_549_1EEB423349A7108C537ABCA51E9947E5` _ragdoll_force_origin_offset) (`PassiveStatBonus_443_2A5E1C3243D6C1E53C6DAD861977ADA2` _passivestatbonus) (`StatusEffect_Settings_524_3ED36F7046947B9246335194B4D1BFCC` _statuseffect_settings) (`SpawnMinions_376_950DA375453D6DEE8971499B1362B3CD` _spawnminions) (`UseAttackSpeed_530_924593E440995ABD3A926EA23A957024` _useattackspeed) (`AttackSpeed_Ratio_535_705AB6FC462DE09448938A82D78F6528` _attackspeed_ratio) (`AttackSpeed_Cast_Cooldown_Ratio_537_DB9B4189470B2D7464177DA4F9094F20` _attackspeed_cast_cooldown_ratio) (`Casting_Settings_526_41EDA36841B326EBBD99DB934FB7EA62` _casting_settings) (`Cooldown_Settings_528_D1E6548447547ADC7624FB833ED68DFC` _cooldown_settings) (`StopMovementOnExecution_370_FAFF9589414AF0A4688573ABC085FD7B` _stopmovementonexecution) (`Overheat_Settings_523_2A805A554E48C38D474B18A68AE2C3E7` _overheat_settings) (`RequiredIWeaponType_460_657FCA154E5CD11D061466AABBD3EAEF` _requirediweapontype) (`Particles_504_0384589D47891C9143D4A4A8E6B24F19` _particles) (`Sound_544_F069E0EE431CAF2DD08C01B63415D0D4` _sound) (`ImpactID_501_1E55FE3D4EF84AFD7E138C9F2F77B170` _impactid) (`SkillModuleClass_440_2D9FF3FB423608B53C1198B2085594B6` _skillmoduleclass) (`DestroyDelay_507_B250641E4F6ECC9C3DED36913A6BFB6C` _destroydelay) (`Icon_439_557516B846326C477D6E7B809F0D1A9A` _icon) (`TraceType_254_9BFE8A074B33E463AEBCF88884F007C0` _tracetype) (`TraceSettings_239_6436F7F74F429B5E93F83AB2033EF85B` _tracesettings) (`BoxTraceSettings_251_A0617A15432F46517C736F8FD2687628` _boxtracesettings)) (break `/Game/RPGSystem/Blueprints/Structure/Skill/S_Skill` (`self.SkillInfo`)))
  (set `self.MaxDamage` _damage)
  (`self.SpawnParticles` "/Game/RPGSystem/Particles/P_Wirbel.P_Wirbel" (struct) (`self.K2_GetActorLocation`) (0.0 0.0 0.0) (2.0 2.0 1.4) (- (* _multihitcount _multihitdelay) 1.8) false self)
  (`self.SkillDoDamage`)
  (`SphereComponent.SetSphereRadius` (`self.Sphere`) (select `/Game/RPGSystem/Blueprints/Enum/Skill/E_SkillTraceType` _tracetype :`NewEnumerator0` (`.Radius_19_6BDBC5774B346A254DE606BFD88AD5E7` (break `/Game/RPGSystem/Blueprints/Structure/Skill/S_SkillSphereTraceSettings` _tracesettings)) :`NewEnumerator1` (`.Length_5_6BDBC5774B346A254DE606BFD88AD5E7` (break `/Game/RPGSystem/Blueprints/Structure/Skill/S_SkillBoxTraceSettings` _boxtracesettings)) :!type "Float (double-precision)") true))

(event `self.OnHitDone`
  (params (Targets :type "Array of /Game/RPGSystem/Blueprints/BPC_RPGSystem Object Reference (by ref)") (StatusEffectTargets :type "Array of /Game/RPGSystem/Blueprints/BPC_RPGSystem Object Reference (by ref)"))
  (bind _maxdamage (`self.MaxDamage`))
  ;[1 1 1] Comment
  (setmembers `/Game/RPGSystem/Blueprints/Structure/Skill/S_Skill` :`StructRef` (`self.SkillInfo`) :`Damage` (`KismetMathLibrary.RandomFloatInRange` (* _maxdamage 0.98) _maxdamage)))

(event `self.ReceiveTick`
  (params (DeltaSeconds :type "Float (single-precision)"))
  (bind _returnvalue (`self.K2_GetActorLocation`))
  (for _array_element (`PrimitiveComponent.GetOverlappingActors` (`self.Sphere`) "/Script/Engine.Actor")
    (bind (_valid _target_) (`/Game/RPGSystem/Blueprints/Utilities/BPL_RPG_Utilities.IsValidTarget` (`self.SkillOwner`) _array_element))
    (if _valid
      (bind _ascharacter (cast `Character` (`ActorComponent.GetOwner` _target_)))
      (bind _radius (message `/Game/RPGSystem/Blueprints/Utilities/BPI_RPG_PlayerCharacter.GetMeshRadius` _ascharacter))
      (bind _returnvalue_2 (`self.K2_GetActorLocation` _ascharacter))
      (bind _returnvalue_3 (`KismetMathLibrary.Vector_Distance` _returnvalue_2 _returnvalue))
      (if (> (- _returnvalue_3 _radius) 100.0)
        (`Character.LaunchCharacter` _ascharacter (* (`KismetMathLibrary.GetForwardVector` (`KismetMathLibrary.FindLookAtRotation` _returnvalue_2 _returnvalue)) (* _returnvalue_3 0.3)) false false)))))

(fn `UserConstructionScript`
  (`parent.UserConstructionScript`))