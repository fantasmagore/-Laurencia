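; BP_SkillParticle_Base is a base actor for skill effects in the RPG system that plays a particle effect and then cleans itself up.
; On BeginPlay it applies the ParticleTemplate to its ParticleSystem component and activates it.
; After DestroyTimer elapses it ends trails and destroys the actor following a short grace delay.
; The system's finished event also destroys the actor, whichever comes first.
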(event `self.ReceiveBeginPlay`
  (bind _particlesystem (`self.ParticleSystem`))
  (`ParticleSystemComponent.SetTemplate` _particlesystem (`self.ParticleTemplate`))
  (`ActorComponent.SetActive` _particlesystem true false)
  (`KismetSystemLibrary.Delay` (`self.DestroyTimer`))
  (`ParticleSystemComponent.EndTrails` (`self.ParticleSystem`))
  (`KismetSystemLibrary.Delay` 2.0)
  (`self.K2_DestroyActor`))

(event `self.ParticleSystem.OnSystemFinished`
  (params (PSystem :type "ParticleSystemComponent Object Reference"))
  (`self.K2_DestroyActor`))

(event `self.ParticleSystem.OnComponentDeactivated`
  (params (Component :type "ActorComponent Object Reference")))

(fn `UserConstructionScript`)