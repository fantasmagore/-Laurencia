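; Bowling Bash skill Blueprint for the Swordman in the RPG skill system.
; On SkillStart it sets the skill's damage from a random roll within the owner's min and max attack, scaled as a percentage of base damage plus a per-level bonus, with a fixed multiplier.
; It then calls either the single-target or area hit function, depending on the targeting type in SkillInfo.
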(event `self.SkillStart`
  (bind _skillinfo (`self.SkillInfo`))
  (bind _skillowner (`self.SkillOwner`))
  (bind ((`AttackType_444_ACFCC5534FFDE6843948798661995027` _attacktype) (`DamageType_447_EE2BF99A40D6A48A6A413B83DA01433D` _damagetype) (`Damage_356_051999E94AC01F21023A41B864B49BC7` _damage) (`CritBonus_448_3B57C4364598C5F583267DB033D55A4F` _critbonus) (`Projectile_Settings_509_A79BB4BB40B6ED6488BE1996BE5FFA52` _projectile_settings) (`Targeting_Settings_511_7CC7E835443906B956308ABA2E8C8EF7` _targeting_settings) (`Spawn_Settings_513_553A9A9A4228718D2171CC868CBDD6C6` _spawn_settings) (`RotateTo_Settings_515_ED859EE64B73CE23997E01B3893AEA09` _rotateto_settings) (`AsyncAttack_Settings_541_5C9CB04444CB3991BAFDDF8D24D390D2` _asyncattack_settings) (`MaxHitTargets_540_0F374CA64BA9FC88F84E1F9C9A12E389` _maxhittargets) (`Trace_Settings_517_9BFE8A074B33E463AEBCF88884F007C0` _trace_settings) (`ShowSkillIndicator_482_774D95804CA28F9C129BCDBAE9E629A8` _showskillindicator) (`Ragdoll_Force_546_D5103DEE45AF6CE66D58DFBCAB5BFA12` _ragdoll_force) (`Ragdoll_Force_Origin_Offset_549_1EEB423349A7108C537ABCA51E9947E5` _ragdoll_force_origin_offset) (`PassiveStatBonus_443_2A5E1C3243D6C1E53C6DAD861977ADA2` _passivestatbonus) (`StatusEffect_Settings_524_3ED36F7046947B9246335194B4D1BFCC` _statuseffect_settings) (`UseAttackSpeed_530_924593E440995ABD3A926EA23A957024` _useattackspeed) (`AttackSpeed_Ratio_535_705AB6FC462DE09448938A82D78F6528` _attackspeed_ratio) (`AttackSpeed_Cast_Cooldown_Ratio_537_DB9B4189470B2D7464177DA4F9094F20` _attackspeed_cast_cooldown_ratio) (`Casting_Settings_526_41EDA36841B326EBBD99DB934FB7EA62` _casting_settings) (`Cooldown_Settings_528_D1E6548447547ADC7624FB833ED68DFC` _cooldown_settings) (`Overheat_Settings_523_2A805A554E48C38D474B18A68AE2C3E7` _overheat_settings) (`RequiredIWeaponType_460_657FCA154E5CD11D061466AABBD3EAEF` _requirediweapontype) (`Particles_504_0384589D47891C9143D4A4A8E6B24F19` _particles) (`Sound_544_F069E0EE431CAF2DD08C01B63415D0D4` _sound) (`ImpactID_501_1E55FE3D4EF84AFD7E138C9F2F77B170` _impactid) (`SkillModuleClass_440_2D9FF3FB423608B53C1198B2085594B6` _skillmoduleclass) (`DestroyDelay_507_B250641E4F6ECC9C3DED36913A6BFB6C` _destroydelay) (`Icon_439_557516B846326C477D6E7B809F0D1A9A` _icon) (`TargetingType_394_7CC7E835443906B956308ABA2E8C8EF7` _targetingtype)) (break `/Game/RPGSystem/Blueprints/Structure/Skill/S_Skill` _skillinfo))
  (setmembers `/Game/RPGSystem/Blueprints/Structure/Skill/S_Skill` :`StructRef` _skillinfo :`Damage` (* (/ (`KismetMathLibrary.Conv_IntToDouble` (`KismetMathLibrary.RandomIntegerInRange` (`KismetMathLibrary.FTrunc` (`/Game/RPGSystem/Blueprints/BPC_RPGSystem.MinATK` _skillowner)) (`KismetMathLibrary.FTrunc` (`/Game/RPGSystem/Blueprints/BPC_RPGSystem.MaxATK` _skillowner)))) 100.0) (* (+ _damage (`KismetMathLibrary.Conv_IntToDouble` (* (`self.SkillLevel`) 40))) 4.0)))
  (if (`|EnumEquality` _targetingtype "NewEnumerator2")
    (`self.HitSingleTarget`)
    (else
      (`self.HitAoe`))))

(fn `UserConstructionScript`
  (`parent.UserConstructionScript`))