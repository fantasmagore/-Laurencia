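; Condemn skill actor that snaps to the ground, spawns a meteor impact and deals level-scaled area damage through inherited skill logic.
; After hits resolve, it waits briefly, then steps through struck targets with a short delayed loop.
; Each living target has a level-based chance to trigger a smaller sphere trace, hitting valid non-owner pawns around it with fire effects.
; The actor destroys itself once the list is exhausted.
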(event `self.SkillStart`
  (bind _skillinfo (`self.SkillInfo`))
  (setmembers `/Game/RPGSystem/Blueprints/Structure/Skill/S_Skill` :`StructRef` _skillinfo :`Damage` (* (+ (`.Damage_356_051999E94AC01F21023A41B864B49BC7` (break `/Game/RPGSystem/Blueprints/Structure/Skill/S_Skill` _skillinfo)) (`KismetMathLibrary.Conv_IntToDouble` (* (`self.SkillLevel`) 40))) (* (`self.SkillLevel`) 0.2)))
  (bind (_returnvalue _location) (`/Game/RPGSystem/Blueprints/Utilities/BPL_RPG_Utilities.FindGround` (`self.K2_GetActorLocation`)))
  (`self.K2_SetActorLocation` _location false true)
  (`self.SpawnParticles` "/Game/RPGSystem/Particles/P_MeteorImpact.P_MeteorImpact" (`self.K2_GetActorRotation`) (`self.K2_GetActorLocation`) (0.0 0.0 0.0) (0.8 0.8 0.8))
  (`self.SkillDoDamage`))

(event `self.SkillEnd`)

(event `self.OnHitDone`
  (params (Targets :type "Array of /Game/RPGSystem/Blueprints/BPC_RPGSystem Object Reference (by ref)") (StatusEffectTargets :type "Array of /Game/RPGSystem/Blueprints/BPC_RPGSystem Object Reference (by ref)"))
  (bind _output (`|GetArrayItem` Targets (`self.OnHitIndex`)))
  (bind _returnvalue (`self.K2_GetActorLocation` (`ActorComponent.GetOwner` _output)))
  (`KismetSystemLibrary.Delay` (`KismetMathLibrary.RandomFloatInRange` 0.15 0.35))
  (if (< (`self.OnHitIndex`) (`KismetArrayLibrary.Array_Length` Targets)) :!label _label
    (if (`KismetSystemLibrary.IsValid` _output)
      (if (`/Game/RPGSystem/Blueprints/BPC_RPGSystem.bIsDead` _output)
        _
        (elif (`/Game/RPGSystem/Blueprints/Utilities/BPL_RPG_Utilities.CalcChance` (* (`self.SkillLevel`) 15.0))
          (bind _outhits (`KismetSystemLibrary.SphereTraceMultiForObjects` _returnvalue _returnvalue (* (`.Radius_19_6BDBC5774B346A254DE606BFD88AD5E7` (break `/Game/RPGSystem/Blueprints/Structure/Skill/S_SkillSphereTraceSettings` (`.TraceSettings_239_6436F7F74F429B5E93F83AB2033EF85B` (break `/Game/RPGSystem/Blueprints/Structure/Skill/S_Skill` (`self.SkillInfo`))))) 0.8) (`|MakeArray` "ObjectTypeQuery3" :!type "EObjectTypeQuery Enum")))
          (for _array_element _outhits
            (bind (_valid _target_) (`/Game/RPGSystem/Blueprints/Utilities/BPL_RPG_Utilities.IsValidTarget` (`self.SkillOwner`) (`.HitActor` (`GameplayStatics.BreakHitResult` _array_element))))
            (if (and _valid (!= (`self.SkillOwner`) _target_))
              (`self.SpawnParticles` "/Game/RPGSystem/Particles/P_Impact_Enemy_Gib_Fire.P_Impact_Enemy_Gib_Fire" (struct) (`self.K2_GetActorLocation` (`ActorComponent.GetOwner` _target_)) (0.0 0.0 0.0) (0.2 0.2 0.1))
              (`self.HitTarget` _target_))))))
    (`/Engine/EditorBlueprintResources/StandardMacros.IncrementInt` (`self.OnHitIndex`)
      (:`  `
        (`KismetSystemLibrary.Delay` 0.08)
        (goto _label)))
    (else
      (`self.K2_DestroyActor`))))

(fn `UserConstructionScript`
  (`parent.UserConstructionScript`))