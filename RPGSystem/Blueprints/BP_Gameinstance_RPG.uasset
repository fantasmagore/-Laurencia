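; RPG system Game Instance that holds custom quest/game variables, global and private per player UniqueID, plus save slot name, cached ServerData and server-travel start tag.
; Init creates and loads ServerData and preloads base classes; Shutdown optionally autosaves.
; Server-gated events edit variables and notify GameMode to replicate changes, fire dispatchers and share listed private variables with parties.
; ServerCV events apply received changes, using a Shared flag to prevent re-sharing.
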(event `self.ReceiveInit`
  ;[1 1 1] Load first ServerData if available
  (bind _return (message `/Game/RPGSystem/Blueprints/Utilities/BPI_GameInstance.GetCurrentSaveName` (`GameplayStatics.GetGameInstance`)))
  (`/Game/RPGSystem/Blueprints/Utilities/BPL_RPG_Utilities.CreateNewServerData` _return) ; Only created on if it doesnt exist
  (`/Game/RPGSystem/Blueprints/Utilities/BPL_RPG_Utilities.LoadServerData` _return)
  (`KismetSystemLibrary.LoadClassAsset_Blocking` "/Game/RPGSystem/Blueprints/Skill/Base/BP_SkillModule_Base.BP_SkillModule_Base_C")
  (`KismetSystemLibrary.LoadClassAsset_Blocking` "/Game/RPGSystem/Blueprints/Item/BP_Item_Base.BP_Item_Base_C")
  (`KismetSystemLibrary.LoadClassAsset_Blocking` "/Game/RPGSystem/Blueprints/Item/Currency/BP_Currency_Item_Base.BP_Currency_Item_Base_C"))

(event `/Game/RPGSystem/Blueprints/Utilities/BPI_RPG_CustomVariable.Server_AddCV`
  (params (Variable :type Name) (Value :type Integer) (UniqueID :type String))
  ;[1 1 1] Receive changes from server
  (if (not (`KismetStringLibrary.IsEmpty` UniqueID))
    (`self.AddCustomVariablePrivate_Function` Variable Value UniqueID true)
    (else
      (`self.AddCustomVariable_Function` Variable Value))))

(event `/Game/RPGSystem/Blueprints/Utilities/BPI_RPG_CustomVariable.AddCustomVariable`
  (params (Variable :type Name) (Value :type Integer) (UniqueID :type String))
  ;[1 1 1] For Server
  (if (`KismetSystemLibrary.IsServer`)
    (if (not (`KismetStringLibrary.IsEmpty` UniqueID))
      (`self.AddCustomVariablePrivate_Function` Variable Value UniqueID)
      (else
        (`self.AddCustomVariable_Function` Variable Value)))))

(event `/Game/RPGSystem/Blueprints/Utilities/BPI_GameInstance.SetSaveObject`
  (params (ServerData :type "/Game/RPGSystem/Blueprints/BPO_ServerData_RPG Object Reference"))
  (set `self.ServerData` ServerData)
  (`/Game/RPGSystem/Blueprints/Utilities/BPL_RPG_Utilities.PrintMessage` "SERVERDATACACHED"))

(event `self.ReceiveShutdown`
  ;[1 1 1] Auto Save on shutdown
  (if (`self.AutoSaveOnClose`)
    (`/Game/RPGSystem/Blueprints/Utilities/BPL_RPG_Utilities.SaveServerData`)))

(event `/Game/RPGSystem/Blueprints/Utilities/BPI_GameInstance.SetCurrentSaveName`
  (params (SaveName :type String))
  (set `self.CurrentSaveName` SaveName))

(event `/Game/RPGSystem/Blueprints/Utilities/BPI_RPG_CustomVariable.Server_RemoveCV`
  (params (Variable :type Name) (UniqueID :type String))
  ;[1 1 1] Receive changes from server
  (if (not (`KismetStringLibrary.IsEmpty` UniqueID))
    (`self.RemoveCustomVariablePrivate_Function` Variable UniqueID)
    (else
      (`self.RemoveCustomVariable_Function` Variable))))

(event `/Game/RPGSystem/Blueprints/Utilities/BPI_RPG_CustomVariable.RemoveCustomVariable`
  (params (Variable :type Name) (UniqueID :type String))
  ;[1 1 1] For Server
  (if (`KismetSystemLibrary.IsServer`)
    (if (not (`KismetStringLibrary.IsEmpty` UniqueID))
      (`self.RemoveCustomVariablePrivate_Function` Variable UniqueID)
      (else
        (`self.RemoveCustomVariable_Function` Variable)))))

(event `/Game/RPGSystem/Blueprints/Utilities/BPI_RPG_CustomVariable.Server_SetCV_Value`
  (params (Variable :type Name) (Value :type Integer) (Add :type Boolean) (UniqueID :type String))
  ;[1 1 1] Receive changes from server
  (if (not (`KismetStringLibrary.IsEmpty` UniqueID))
    (`self.SetCustomVariableValuePrivate_Function` Variable Value Add UniqueID true)
    (else
      (`self.SetCustomVariableValue_Function` Variable Value Add))))

(event `/Game/RPGSystem/Blueprints/Utilities/BPI_RPG_CustomVariable.SetCustomVariableValue`
  (params (Variable :type Name) (Value :type Integer) (Add :type Boolean) (UniqueID :type String))
  ;[1 1 1] For Server
  (if (`KismetSystemLibrary.IsServer`)
    (if (not (`KismetStringLibrary.IsEmpty` UniqueID))
      (`self.SetCustomVariableValuePrivate_Function` Variable Value Add UniqueID)
      (else
        (`self.SetCustomVariableValue_Function` Variable Value Add)))))

(event `/Game/RPGSystem/Blueprints/Utilities/BPI_RPG_CustomVariable.SetAllCustomVariablePrivateByUniqueID`
  (params (UniqueID :type String) (CustomVariablePrivate :type "/Game/RPGSystem/Blueprints/Structure/CustomVariable/S_CustomVariable_Array2D Structure"))
  ;[1 1 1] Save System | Client
  (`BlueprintMapLibrary.Map_Add` (`self.CustomVariablePrivate`) UniqueID CustomVariablePrivate))

(event `/Game/RPGSystem/Blueprints/Utilities/BPI_RPG_CustomVariable.SetAllCustomVariable_FromServer`
  (params (Variables :type "Array of Name (by ref)") (Values :type "Array of Integer (by ref)"))
  ;[1 1 1] Save System | Client
  (`BlueprintMapLibrary.Map_Clear` (`self.CustomVariable`))
  (for (_array_element _array_index) Variables
    (`BlueprintMapLibrary.Map_Add` (`self.CustomVariable`) _array_element (`|GetArrayItem` Values _array_index))))

(event `/Game/RPGSystem/Blueprints/Utilities/BPI_RPG_CustomVariable.SetAllCustomVariable`
  (params (Variables :type "Map of Name to Integer"))
  ;[1 1 1] Save System | Server-side
  (set `self.CustomVariable` Variables))

(event `/Game/RPGSystem/Blueprints/Utilities/BPI_RPG_CustomVariable.SetAllCustomVariablePrivate`
  (params (VariablesPrivate :type "Map of String to /Game/RPGSystem/Blueprints/Structure/CustomVariable/S_CustomVariable_Array2D Structure"))
  ;[1 1 1] Save System | Server-side
  (set `self.CustomVariablePrivate` VariablesPrivate))

(event `ApplyGlobalSettings_1`
  (params (Settings :type "/Game/RPGSystem/Blueprints/Structure/Settings/S_Settings Structure")))

(event `/Game/RPGSystem/Blueprints/Utilities/BPI_GameInstance.SetServerTravelStartPointTag`
  (params (Tag :type Name))
  (set `self.ServerTravelStartPointTag` Tag))

(fn `AddCustomVariable_Function`
  (params (Variable :type Name) (Value :type Integer))
  (locals (VarUniqueID :type Name))
  (`BlueprintMapLibrary.Map_Add` (`self.CustomVariable`) (`local.Variable`) (`local.Value`))
  (if (`KismetSystemLibrary.IsServer`)
    (`|ExecutionSequence`
      (:`then_0`
        (message `/Game/RPGSystem/Blueprints/Utilities/BPI_RPG_CustomVariable.Server_AddCV` (`GameplayStatics.GetGameMode`) (`local.Variable`) (`local.Value`) ""))
      (:`then_1`
        (message `/Game/RPGSystem/Blueprints/Utilities/BPI_RPG_GameMode.CallCustomDispatcherVariable` (`GameplayStatics.GetGameMode`) (`local.Variable`) (`local.Value`) false "")))))

(fn `AddCustomVariablePrivate_Function`
  (params (Variable :type Name) (Value :type Integer) (UniqueID :type String) (Shared :type Boolean))
  (locals (VarValue :type "/Game/RPGSystem/Blueprints/Structure/CustomVariable/S_CustomVariable_Array2D Structure"))
  (bind _output_get (set `local.VarValue` (`BlueprintMapLibrary.Map_Find` (`self.CustomVariablePrivate`) UniqueID)))
  (bind (_variables _values) (break `/Game/RPGSystem/Blueprints/Structure/CustomVariable/S_CustomVariable_Array2D` _output_get))
  (if (not (`KismetArrayLibrary.Array_Contains` _variables (`local.Variable`)))
    (`KismetArrayLibrary.Array_Add` _variables (`local.Variable`))
    (`KismetArrayLibrary.Array_Add` _values (`local.Value`))
    (`BlueprintMapLibrary.Map_Add` (`self.CustomVariablePrivate`) UniqueID (`local.VarValue`))
    (if (`KismetSystemLibrary.IsServer`)
      (`|ExecutionSequence`
        (:`then_0`
          (message `/Game/RPGSystem/Blueprints/Utilities/BPI_RPG_CustomVariable.Server_AddCV` (`GameplayStatics.GetGameMode`) (`local.Variable`) (`local.Value`) (`local.UniqueID`))
          (bind (_success _reference) (`/Game/RPGSystem/Blueprints/Utilities/BPL_RPG_Utilities.GetPlayerByUniqueID` (`local.UniqueID`)))
          (if _success
            (if (and (not (`local.Shared`)) (`KismetArrayLibrary.Array_Contains` (`/Game/RPGSystem/Blueprints/BPC_RPGSystem.VariablesToShare` _reference) (`local.Variable`)))
              (message `/Game/RPGSystem/Blueprints/Utilities/BPI_RPG_GameMode.Server_SharePrivateVariable` (`GameplayStatics.GetGameMode`) (`|MakeArray` (`local.Variable`)) (`local.Value`) true (`local.UniqueID`) (`/Game/RPGSystem/Blueprints/BPC_RPGSystem.PartyID` _reference)))))
        (:`then_1`
          (message `/Game/RPGSystem/Blueprints/Utilities/BPI_RPG_GameMode.CallCustomDispatcherVariable` (`GameplayStatics.GetGameMode`) (`local.Variable`) (`local.Value`) true (`local.UniqueID`)))))))

(fn `GetAccountName`
  (returns (Return :type Text))
  (bind _uniqueid (`self.GetLocalUniqueNetID`))
  (return (`KismetTextLibrary.Conv_StringToText` _uniqueid)))

(fn `GetAllCustomVariable`
  (returns (CustomVariable :type "/Game/RPGSystem/Blueprints/Structure/CustomVariable/S_All_CustomVariable Structure"))
  (return (make `/Game/RPGSystem/Blueprints/Structure/CustomVariable/S_All_CustomVariable` (`self.CustomVariable`) (`self.CustomVariablePrivate`))))

(fn `GetAllCustomVariablePrivateByUniqueID`
  (params (UniqueID :type String))
  (returns (CustomVariablePrivate :type "/Game/RPGSystem/Blueprints/Structure/CustomVariable/S_CustomVariable_Array2D Structure"))
  (return (`BlueprintMapLibrary.Map_Find` (`self.CustomVariablePrivate`) UniqueID)))

(fn `GetAutosaveOnClosing`
  (returns (Return :type Boolean))
  (return (`self.AutoSaveOnClose`)))

(fn `GetCurrentCharacterIndex`
  (returns (Index :type Integer))
  (return 0))

(fn `GetCurrentSaveName`
  (returns (Return :type String))
  (return (`self.CurrentSaveName`)))

(fn `GetCustomVariableValue`
  (params (Variable :type Name) (UniqueID :type String))
  (returns (Success :type Boolean) (Value :type Integer))
  (locals (VarIndex :type Integer))
  (bind (_value _returnvalue) (`BlueprintMapLibrary.Map_Find` (`self.CustomVariable`) Variable))
  (bind (_value_2 _returnvalue_2) (`BlueprintMapLibrary.Map_Find` (`self.CustomVariablePrivate`) (`local.UniqueID`)))
  (bind (_variables _values) (break `/Game/RPGSystem/Blueprints/Structure/CustomVariable/S_CustomVariable_Array2D` _value_2))
  (if (`KismetStringLibrary.IsEmpty` UniqueID)
    (if _returnvalue
      (return true _value)
      (else
        (return false 0)))
    (elif _returnvalue_2
      (bind _output_get (set `local.VarIndex` (`KismetArrayLibrary.Array_Find` _variables Variable)))
      (if (!= _output_get -1)
        (return true (`|GetArrayItem` _values (`local.VarIndex`)))
        (else
          (return false 0)))
      (else
        (return false 0)))))

(fn `GetLocalUniqueNetID`
  (returns (UniqueID :type String))
  (return ""))

(fn `GetSaveObject`
  (returns (Return :type "/Game/RPGSystem/Blueprints/BPO_ServerData_RPG Object Reference"))
  (return (`self.ServerData`)))

(fn `GetServerTravelStartPointTag`
  (returns (Return :type Name))
  (return (`self.ServerTravelStartPointTag`)))

(fn `RemoveCustomVariable_Function`
  (params (Variable :type Name))
  (locals (VarUniqueID :type Name))
  (`BlueprintMapLibrary.Map_Remove` (`self.CustomVariable`) (`local.Variable`))
  (if (`KismetSystemLibrary.IsServer`)
    (if (`KismetSystemLibrary.IsDedicatedServer`)
      (message `/Game/RPGSystem/Blueprints/Utilities/BPI_RPG_CustomVariable.Server_RemoveCV` (`GameplayStatics.GetGameMode`) (`local.Variable`) "")
      (else
        (message `/Game/RPGSystem/Blueprints/Utilities/BPI_RPG_CustomVariable.Server_RemoveCV` (`GameplayStatics.GetGameMode`) (`local.Variable`) "")
        (bind (_success _reference) (message `/Game/RPGSystem/Blueprints/Utilities/BPI_RPG_PlayerCharacter.GetRPGSystem` (`GameplayStatics.GetPlayerCharacter` 0)))
        (`/Game/RPGSystem/Blueprints/BPC_RPGSystem.UpdateQuestTask` _reference (`local.Variable`) -1 false)))))

(fn `RemoveCustomVariablePrivate_Function`
  (params (Variable :type Name) (UniqueID :type String))
  (locals (VarValue :type "/Game/RPGSystem/Blueprints/Structure/CustomVariable/S_CustomVariable_Array2D Structure") (VarIndex :type Integer))
  (bind (_varvalue_variables _varvalue_values) (break `/Game/RPGSystem/Blueprints/Structure/CustomVariable/S_CustomVariable_Array2D` (`local.VarValue`)))
  (bind _varindex (`local.VarIndex`))
  (bind (_value _returnvalue) (`BlueprintMapLibrary.Map_Find` (`self.CustomVariablePrivate`) UniqueID))
  (if _returnvalue
    (bind _output_get (set `local.VarValue` _value))
    (bind _output_get_2 (set `local.VarIndex` (`KismetArrayLibrary.Array_Find` (`.Variables_9_F584B61846F2FCF33FE953995FF5BB0C` (break `/Game/RPGSystem/Blueprints/Structure/CustomVariable/S_CustomVariable_Array2D` _output_get)) (`local.Variable`))))
    (if (!= _output_get_2 -1)
      (`KismetArrayLibrary.Array_Remove` _varvalue_variables _varindex)
      (`KismetArrayLibrary.Array_Remove` _varvalue_values _varindex)
      (`BlueprintMapLibrary.Map_Add` (`self.CustomVariablePrivate`) (`local.UniqueID`) (`local.VarValue`))
      (if (`KismetSystemLibrary.IsServer`)
        (message `/Game/RPGSystem/Blueprints/Utilities/BPI_RPG_CustomVariable.Server_RemoveCV` (`GameplayStatics.GetGameMode`) (`local.Variable`) (`local.UniqueID`))))))

(fn `SetCustomVariableValue_Function`
  (params (Variable :type Name) (Value :type Integer) (Add :type Boolean))
  (locals (VarUniqueID :type Name) (VarNewValue :type Integer))
  (bind _value (`local.Value`))
  (bind (_value_2 _returnvalue) (`BlueprintMapLibrary.Map_Find` (`self.CustomVariable`) Variable))
  (if _returnvalue
    (set `local.VarNewValue` (select `bool` (`local.Add`) :`false` _value :`true` (+ _value _value_2)))
    (`BlueprintMapLibrary.Map_Add` (`self.CustomVariable`) (`local.Variable`) (`local.VarNewValue`))
    (if (`KismetSystemLibrary.IsServer`)
      (`|ExecutionSequence`
        (:`then_0`
          (message `/Game/RPGSystem/Blueprints/Utilities/BPI_RPG_CustomVariable.Server_SetCV_Value` (`GameplayStatics.GetGameMode`) (`local.Variable`) (`local.VarNewValue`) false ""))
        (:`then_1`
          (message `/Game/RPGSystem/Blueprints/Utilities/BPI_RPG_GameMode.CallCustomDispatcherVariable` (`GameplayStatics.GetGameMode`) (`local.Variable`) (`local.VarNewValue`) false ""))))))

(fn `SetCustomVariableValuePrivate_Function`
  (params (Variable :type Name) (Value :type Integer) (Add :type Boolean) (UniqueID :type "String (by ref)") (Shared :type Boolean))
  (locals (VarUniqueID :type Name) (VarValue :type "/Game/RPGSystem/Blueprints/Structure/CustomVariable/S_CustomVariable_Array2D Structure") (VarIndex :type Integer :default 0) (VarNewValue :type Integer))
  (bind _value (`local.Value`))
  (if (not (`KismetStringLibrary.IsEmpty` UniqueID))
    (bind _output_get (set `local.VarValue` (`BlueprintMapLibrary.Map_Find` (`self.CustomVariablePrivate`) (`local.UniqueID`))))
    (bind (_variables _values) (break `/Game/RPGSystem/Blueprints/Structure/CustomVariable/S_CustomVariable_Array2D` _output_get))
    (bind _output_get_2 (set `local.VarIndex` (`KismetArrayLibrary.Array_Find` _variables (`local.Variable`))))
    (if (!= _output_get_2 -1)
      (bind _output (`|GetArrayItem` _values (`local.VarIndex`)))
      (set `local.VarNewValue` (select `bool` (`local.Add`) :`false` _value :`true` (+ _value _output)))
      (`|VariableSetRef` _output (`local.VarNewValue`))
      (`BlueprintMapLibrary.Map_Add` (`self.CustomVariablePrivate`) (`local.UniqueID`) (`local.VarValue`))
      (if (`KismetSystemLibrary.IsServer`)
        (`|ExecutionSequence`
          (:`then_0`
            (message `/Game/RPGSystem/Blueprints/Utilities/BPI_RPG_CustomVariable.Server_SetCV_Value` (`GameplayStatics.GetGameMode`) (`local.Variable`) (`local.Value`) (`local.Add`) (`local.UniqueID`))
            (bind (_success _reference) (`/Game/RPGSystem/Blueprints/Utilities/BPL_RPG_Utilities.GetPlayerByUniqueID` (`local.UniqueID`)))
            (if _success
              (if (and (not (`local.Shared`)) (`KismetArrayLibrary.Array_Contains` (`/Game/RPGSystem/Blueprints/BPC_RPGSystem.VariablesToShare` _reference) (`local.Variable`)))
                (message `/Game/RPGSystem/Blueprints/Utilities/BPI_RPG_GameMode.Server_SharePrivateVariable` (`GameplayStatics.GetGameMode`) (`|MakeArray` (`local.Variable`)) (`local.Value`) (`local.Add`) (`local.UniqueID`) (`/Game/RPGSystem/Blueprints/BPC_RPGSystem.PartyID` _reference)))))
          (:`then_1`
            (message `/Game/RPGSystem/Blueprints/Utilities/BPI_RPG_GameMode.CallCustomDispatcherVariable` (`GameplayStatics.GetGameMode`) (`local.Variable`) (`local.VarNewValue`) true (`local.UniqueID`))))))))