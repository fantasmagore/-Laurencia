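; Base Blueprint for currency item pickups, showing a coin mesh and tinting particles gold once the mesh finishes loading.
; For persistent items with visual setup enabled, the construction script looks up the item's data table row by ID.
; Larger amounts raise the random chance of the medium coin mesh replacing the row's default mesh.
; It loads the mesh synchronously, creates a component if needed, applies the row's offset and calls the load-finished event.
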(event `self.OnAsyncLoadStaticMeshFinished`
  (`parent.OnAsyncLoadStaticMeshFinished`)
  (`self.SetParticleColor` (struct :`R` 1.0 :`G` 0.878431 :`A` 1.0)))

(fn `UserConstructionScript`
  (locals (VarMeshToLoad :type "Object Soft Object Reference"))
  (bind _visualstaticmeshcomponent (`self.VisualStaticMeshComponent`))
  (if (`self.Persistant`)
    (if (not (`self.bDisableVisualSetup`))
      (bind _returnvalue (`|GetDataTableRow` (`self.Item_DT`) (`.ItemID_73_6C4D3C2D4D49AA75490544AC57C7939B` (break `/Game/RPGSystem/Blueprints/Structure/Inventory/S_Inventory` (`self.Item`))))
        (:`then`
          (bind ((`StaticMesh_10_5AF351D148CFDE3F574A5B90C1BEFA8A` _staticmesh) (`MeshOffset_12_74C83F31405A4049950A72A118CC1DB4` _meshoffset)) (break `/Game/RPGSystem/Blueprints/Structure/Item/S_Item_BlueprintDrop_Settings` (`.BlueprintSettings_465_835AD89D44481B6D40315E9B17E116F0` (break `/Game/RPGSystem/Blueprints/Structure/Item/S_Item` _returnvalue))))
          (set `local.VarMeshToLoad` (select `bool` (`KismetMathLibrary.RandomBoolWithWeight` (`KismetMathLibrary.MapRangeClamped` (`KismetMathLibrary.Conv_IntToDouble` (`.Amount_79_18AF9F2D4F0C4D2C11058F8B990FAC86` (break `/Game/RPGSystem/Blueprints/Structure/Inventory/S_Inventory` (`self.Item`)))) 200.0 2000.0 0.1 1.0)) :`false` _staticmesh :`true` "/Game/RPGSystem/Models/GoldCoin/Mesh/SM_Coin_Medium.SM_Coin_Medium" :!type "Object Soft Object Reference"))
          (if (`KismetSystemLibrary.IsValidSoftObjectReference` (`local.VarMeshToLoad`))
            (bind _returnvalue_2 (`KismetSystemLibrary.LoadAsset_Blocking` (`local.VarMeshToLoad`)))
            (bind _asstatic_mesh (cast `StaticMesh` _returnvalue_2))
            (`/Engine/EditorBlueprintResources/StandardMacros.IsValid` (`self.VisualStaticMeshComponent`)
              (:`Is Valid`
                _)
              (:`Is Not Valid`
                (bind _returnvalue_3 (`AddComponent|NODE_AddStaticMeshComponent-0`))
                (set `self.DefaultSceneRoot` _returnvalue_3)
                (set `self.VisualStaticMeshComponent` _returnvalue_3)))
            (`StaticMeshComponent.SetStaticMesh` _visualstaticmeshcomponent _asstatic_mesh)
            (`SceneComponent.K2_SetRelativeTransform` _visualstaticmeshcomponent _meshoffset false true)
            (`self.OnAsyncLoadStaticMeshFinished`)))))))