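; Base world item pickup for the RPG system, either placed (Persistant) or dropped, that players interact with to loot.
; Item data table rows drive name, rarity color and mesh, loaded blocking in construction for placed items or async for drops.
; Meshes launch with physics, arcing toward any LandPosition, then dampen and play a rarity sound on impact.
; The server handles inventory transfer and leftover stacks, while RepNotifies refresh appearance and hide grabbed items on clients.
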(event `OnAsyncLoadStaticMeshFinished`
  (bind _rarityparticle (`self.RarityParticle`))
  ;[1 1 1] OnAsyncLoadStaticMeshFinished
  (`self.CheckEnablePhysic`)
  (`/Engine/EditorBlueprintResources/StandardMacros.IsValid` _rarityparticle
    (:`Is Valid`
      (`SceneComponent.K2_AttachToComponent` _rarityparticle (`self.PhysicComp`) "None" "SnapToTarget" "KeepRelative" "KeepRelative" false))))

(event `LoadtStaticMeshAsync`
  (params (StaticMesh :type "StaticMesh Soft Object Reference") (NewTransform :type "Transform Structure (by ref)"))
  ;[0.2083 1 1] Load Visual Static Mesh Async
  (if (`KismetSystemLibrary.IsValidSoftObjectReference` StaticMesh)
    (`|LoadAsset` StaticMesh
      (:`Completed`
        (`self.InitVisualMesh` (`|ConvertAsset` StaticMesh) NewTransform)
        (`self.OnAsyncLoadStaticMeshFinished`)))
    (else
      (`self.CheckEnablePhysic`))))

(event `OnHit`
  (params (HitComponent :type "PrimitiveComponent Object Reference") (OtherActor :type "Actor Object Reference") (OtherComp :type "PrimitiveComponent Object Reference") (NormalImpulse :type "Vector Structure") (Hit :type "HitResult Structure (by ref)"))
  ;[1 1 1] On Hit Event - Fire ItemType Specific Drop Sound
  (`PrimitiveComponent.SetNotifyRigidBodyCollision` HitComponent false)
  (remove `PrimitiveComponent.OnComponentHit` HitComponent (delegate `OnHit`))
  (`ActorComponent.SetActive` (`self.RarityParticle`) true false)
  (`PrimitiveComponent.SetPhysicsLinearVelocity` HitComponent (* (`SceneComponent.GetComponentVelocity` HitComponent) 0.1) false "None")
  (`PrimitiveComponent.SetPhysicsAngularVelocityInDegrees` HitComponent (* (`PrimitiveComponent.GetPhysicsAngularVelocityInDegrees` HitComponent "None") 0.1) false "None")
  (`self.PlayRarityDropSound`))

(event `self.ReceiveBeginPlay`
  ;[1 1 1] Begin Play
  (`|ExecutionSequence`
    (:`then_0`
      (`/Engine/EditorBlueprintResources/ActorMacros.Switch Has Authority`
        (:`Authority`
          (if (`self.Persistant`)
            (bind (_success _inventory_struct) (`/Game/RPGSystem/Blueprints/Utilities/BPL_RPG_Utilities.CreateItem` (`self.Item`)))
            (set `self.Item` _inventory_struct)
            (set `self.NewDrop` true)))))
    (:`then_1`
      (bind _iteminfo (`self.InitItemInfo`))
      (if (`self.Persistant`)
        (bind ((`Category_152_F5F888424D2DCDC29859AB8E5E1F0D47` _category) (`EquipmentSetID_492_F3CF6A5F4135E759D1E70E9AC03925E2` _equipmentsetid)) (break `/Game/RPGSystem/Blueprints/Structure/Item/S_Item` _iteminfo))
        (`self.SetParticleColor` (`/Game/RPGSystem/Blueprints/Utilities/BPL_RPG_Utilities.Get Rarity Color` (`.Rarity_78_C81B885D4BCDFA0088309599CDCB283C` (break `/Game/RPGSystem/Blueprints/Structure/Inventory/S_Inventory` (`self.Item`))) (!= _equipmentsetid "None")))
        (else
          (`self.SetupAppearance` _iteminfo)
          (if (or (`|EnumEquality` _category "NewEnumerator1") (`|EnumEquality` _category "NewEnumerator2") (`self.FromInventory`))
            (`GameplayStatics.SpawnSoundAtLocation` "/Game/RPGSystem/Sound/Item/SC_ItemDrop.SC_ItemDrop" (`self.K2_GetActorLocation`) (struct) 1.0 1.0 0.0 "/Game/RPGSystem/Sound/Attenuation/SA_ItemDrop.SA_ItemDrop" "/Game/RPGSystem/Sound/Attenuation/ItemDrop_Concurrency.ItemDrop_Concurrency")))))
    (:`then_2`
      (set `self.Created` true))))

(event `/Game/RPGSystem/Blueprints/Utilities/BPI_RPG_Interaction.Interact`
  (params (Player :type "/Game/RPGSystem/Blueprints/BPC_RPGSystem Object Reference") (Command :type String))
  ;[1 1 1] Interact
  (`/Engine/EditorBlueprintResources/StandardMacros.IsValid` Player
    (:`Is Valid`
      (`/Engine/EditorBlueprintResources/ActorMacros.Switch Has Authority`
        (:`Authority`
          (if (`self.Persistant`)
            (if (`self.Created`)
              (bind (_global _private) (`self.GetCustomVariables` :!label _label))
              (bind (_success _stackleft) (`/Game/RPGSystem/Blueprints/BPC_RPGSystem.InventoryAddItem` Player (`self.Item`) _global _private))
              (if _success
                (if (> _stackleft 0)
                  (setmembers `/Game/RPGSystem/Blueprints/Structure/Inventory/S_Inventory` :`StructRef` (`self.Item`) :`Amount` _stackleft)
                  (`self.InitItemInfo`)
                  (else
                    (`self.OnLooted`)
                    (`self.K2_DestroyActor`)))))
            (else
              (goto _label))))))))

(event `/Game/RPGSystem/Blueprints/Utilities/BPI_RPG_Interaction.SelectInteractable`
  (params (Selected :type Boolean))
  ;[1 1 1] Outline
  (if (`KismetSystemLibrary.IsValid` (`self.VisualStaticMeshComponent`))
    (`PrimitiveComponent.SetRenderCustomDepth` (`self.VisualStaticMeshComponent`) Selected)))

(fn `CheckEnablePhysic`
  (bind _returnvalue (`self.GetComponentByClass` "/Script/Engine.StaticMeshComponent"))
  (bind _physiccomp (`self.PhysicComp`))
  (if (`self.EnablePhysic`)
    (`/Engine/EditorBlueprintResources/StandardMacros.IsValid` (`self.PhysicComp`)
      (:`Is Valid`
        _)
      (:`Is Not Valid`
        ;[0 0 0] Search for a Static Mesh
        (`/Engine/EditorBlueprintResources/StandardMacros.IsValid` _returnvalue
          (:`Is Valid`
            (set `self.PhysicComp` _returnvalue))
          (:`Is Not Valid`
            ;[0 0 0] Add a Box Collision if no StaticMesh is present and EnablePhysic is set to true - Box draw is not hidden ingame
            (bind _returnvalue_2 (`AddComponent|NODE_AddBoxComponent-0`))
            (set `self.PhysicComp` _returnvalue_2)))))
    ;[0 0 0] Enable Simulate Physic
    (if (not (`SceneComponent.IsAnySimulatingPhysics` _physiccomp))
      (`SceneComponent.K2_SetWorldRotation` _physiccomp (`KismetMathLibrary.RandomRotator` false) false false)
      (`PrimitiveComponent.SetSimulatePhysics` (`self.PhysicComp`) true))))

(fn `GetCustomVariables`
  (returns (Global :type "/Game/RPGSystem/Blueprints/Structure/Misc/S_ArrayOf_FName Structure") (Private :type "/Game/RPGSystem/Blueprints/Structure/Misc/S_ArrayOf_FName Structure"))
  (locals (VarCustomVariables :type "Array of Name") (VarCustomVariablesPrivate :type "Array of Name"))
  (bind (_global _private _globaltag _privatetag) (break `/Game/RPGSystem/Blueprints/Structure/CustomVariable/S_CustomVariable_OnExpose` (`self.CustomVariables`)))
  (set `local.VarCustomVariables` _global)
  (set `local.VarCustomVariablesPrivate` _private)
  (for _array_element _globaltag
    (`KismetArrayLibrary.Array_Add` (`local.VarCustomVariables`) (`BlueprintGameplayTagLibrary.GetTagName` _array_element)))
  (for _array_element_2 _privatetag
    (`KismetArrayLibrary.Array_Add` (`local.VarCustomVariablesPrivate`) (`BlueprintGameplayTagLibrary.GetTagName` _array_element_2)))
  (return (make `/Game/RPGSystem/Blueprints/Structure/Misc/S_ArrayOf_FName` (`local.VarCustomVariables`)) (make `/Game/RPGSystem/Blueprints/Structure/Misc/S_ArrayOf_FName` (`local.VarCustomVariablesPrivate`))))

(fn `GetInteractableComponents`
  (returns (Components :type "Array of PrimitiveComponent Object Reference"))
  (return))

(fn `GetInteractInfo`
  (params (Player :type "/Game/RPGSystem/Blueprints/BPC_RPGSystem Object Reference"))
  (returns (Success :type Boolean) (Type :type "/Game/RPGSystem/Blueprints/Enum/Interact/E_InteractType Enum") (Action :type "/Game/RPGSystem/Blueprints/Enum/Interact/E_InteractAction Enum"))
  (locals (VarGoal :type "Vector Structure" :default (0.0 0.0 0.0)))
  (bind _returnvalue (`ActorComponent.GetOwner` Player))
  (bind _returnvalue_2 (`self.K2_GetActorLocation` _returnvalue))
  (bind _range (message `/Game/RPGSystem/Blueprints/Utilities/BPI_RPG_PlayerController.GetInteractionRange` (`self.GetInstigatorController` _returnvalue)))
  (bind (_radius _halfheight) (message `/Game/RPGSystem/Blueprints/Utilities/BPI_RPG_PlayerCharacter.GetMeshRadius` _returnvalue))
  (bind _worldlocation (`self.GetMoveToEndDestination` (`local.Player`)))
  (if (<= (`/Game/RPGSystem/Blueprints/Utilities/BPL_RPG_Utilities.GetDistanceExt` _worldlocation _returnvalue_2 _radius (* _halfheight 2.0)) _range)
    (bind _return (`self.GetLookAtLocation`))
    (if (`/Game/RPGSystem/Blueprints/Utilities/BPL_RPG_Utilities.IsTargetInAngle` _return _returnvalue_2 (`self.GetActorForwardVector` (`ActorComponent.GetOwner` (`local.Player`))) 45.0)
      (return true "NewEnumerator0" "NewEnumerator0")
      (else
        (return true "NewEnumerator0" "NewEnumerator5")))
    (else
      (return true "NewEnumerator0" "NewEnumerator1"))))

(fn `GetItemInfo`
  (returns (Success :type Boolean) (Item :type "/Game/RPGSystem/Blueprints/Structure/Inventory/S_Inventory Structure") (ItemType :type "/Game/RPGSystem/Blueprints/Enum/Item/E_ItemType Enum") (CustomVariables :type "/Game/RPGSystem/Blueprints/Structure/Misc/S_ArrayOf_FName Structure") (CustomVariablesPrivate :type "/Game/RPGSystem/Blueprints/Structure/Misc/S_ArrayOf_FName Structure"))
  (locals (VarCustomVariables :type "Array of Name"))
  (bind (_global _private) (`self.GetCustomVariables`))
  (return true (`self.Item`) (`self.ItemType`) _global _private))

(fn `GetLookAtLocation`
  (returns (Return :type "Vector Structure"))
  (`/Engine/EditorBlueprintResources/StandardMacros.IsValid` (`self.VisualStaticMeshComponent`)
    (:`Is Valid`
      (return (`SceneComponent.K2_GetComponentLocation` (`self.VisualStaticMeshComponent`))))
    (:`Is Not Valid`
      (return (+ (`self.K2_GetActorLocation`) (0.0 0.0 40.0))))))

(fn `GetMoveToEndDestination`
  (params (Player :type "/Game/RPGSystem/Blueprints/BPC_RPGSystem Object Reference"))
  (returns (WorldLocation :type "Vector Structure"))
  (locals (VarLoc :type "Vector Structure" :default (0.0 0.0 0.0)) (VaBound :type "Float (double-precision)" :default 0.0))
  (bind (_origin _boxextent _sphereradius) (`KismetSystemLibrary.GetComponentBounds` (`self.VisualStaticMeshComponent`)))
  (`/Engine/EditorBlueprintResources/StandardMacros.IsValid` (`self.VisualStaticMeshComponent`)
    (:`Is Valid`
      (set `local.VarLoc` _origin)
      (set `local.VaBound` _sphereradius))
    (:`Is Not Valid`
      (set `local.VarLoc` (`self.K2_GetActorLocation`))
      (set `local.VaBound` 0.0)))
  (return (+ (`local.VarLoc`) (* (`KismetMathLibrary.GetForwardVector` (`KismetMathLibrary.MakeRotator` 0.0 0.0 (.yaw (`KismetMathLibrary.FindLookAtRotation` (`local.VarLoc`) (`self.K2_GetActorLocation` (`ActorComponent.GetOwner` Player)))))) (`local.VaBound`)))))

(fn `GetScreenTooltipInfo`
  (params (Player :type "/Game/RPGSystem/Blueprints/BPC_RPGSystem Object Reference"))
  (returns (Success :type Boolean) (Text :type Text) (Color :type "LinearColor Structure"))
  (bind (_success _type _action) (`self.GetInteractInfo` Player))
  (return true (select `/Game/RPGSystem/Blueprints/Enum/Interact/E_InteractAction` _action :`NewEnumerator0` "Pickup [E]" :`NewEnumerator1` "Too far away" :!type "Text") (struct :`R` 1.0 :`G` 1.0 :`B` 1.0 :`A` 1.0)))

(fn `GetTeamID`
  (returns (Return :type String))
  (return ""))

(fn `GetWorldTooltipInfo`
  (params (HitComp :type "PrimitiveComponent Object Reference"))
  (returns (Success :type Boolean) (Interactable :type Boolean) (Text :type Text) (Color :type "LinearColor Structure") (Offset :type "Vector Structure"))
  (return true true (`self.ItemName`) (struct) (0.0 0.0 0.0)))

(fn `InitItemInfo`
  (returns (ItemInfo :type "/Game/RPGSystem/Blueprints/Structure/Item/S_Item Structure"))
  (bind ((`RefineLevel_21_4EAA20D34D5B40D6737F4D9B8528182B` _refinelevel) (`Rarity_78_C81B885D4BCDFA0088309599CDCB283C` _rarity) (`Amount_79_18AF9F2D4F0C4D2C11058F8B990FAC86` _amount)) (break `/Game/RPGSystem/Blueprints/Structure/Inventory/S_Inventory` (`self.Item`)))
  (bind _returnvalue (`|GetDataTableRow` (`self.Item_DT`) (`.ItemID_73_6C4D3C2D4D49AA75490544AC57C7939B` (break `/Game/RPGSystem/Blueprints/Structure/Inventory/S_Inventory` (`self.Item`))))
    (:`then`
      (set `self.ItemInfo` _returnvalue)
      (set `self.ItemName` (`/Game/RPGSystem/Blueprints/Utilities/BPL_RPG_Utilities.GetItemName` _returnvalue _rarity _refinelevel _amount true "WorldTooltip_"))
      (return (`self.ItemInfo`)))))

(fn `InitVisualMesh`
  (params (Mesh :type "StaticMesh Object Reference") (Relative :type "Transform Structure (by ref)"))
  (bind _visualstaticmeshcomponent (`self.VisualStaticMeshComponent`))
  (`/Engine/EditorBlueprintResources/StandardMacros.IsValid` (`self.VisualStaticMeshComponent`)
    (:`Is Valid`
      _)
    (:`Is Not Valid`
      (bind _returnvalue (`AddComponent|NODE_AddStaticMeshComponent-4`))
      (set `self.VisualStaticMeshComponent` _returnvalue)))
  (bind _returnvalue_2 (`StaticMeshComponent.SetStaticMesh` _visualstaticmeshcomponent Mesh))
  (if _returnvalue_2
    (`SceneComponent.K2_SetRelativeTransform` (`self.VisualStaticMeshComponent`) Relative false true)
    (add `PrimitiveComponent.OnComponentHit` _visualstaticmeshcomponent (`|CreateDelegate` :!event `OnHit`))
    (if (`KismetMathLibrary.NotEqualExactly_VectorVector` (`self.LandPosition`))
      (bind _outlaunchvelocity (`GameplayStatics.SuggestProjectileVelocity_CustomArc` (`SceneComponent.K2_GetComponentLocation` (`self.VisualStaticMeshComponent`)) (`self.LandPosition`) 0.0 0.2))
      (`PrimitiveComponent.SetPhysicsLinearVelocity` (`self.VisualStaticMeshComponent`) _outlaunchvelocity false "None")
      (else
        (`PrimitiveComponent.SetPhysicsLinearVelocity` (`self.VisualStaticMeshComponent`) (* (+ (* (`self.GetActorForwardVector`) 0.8) (* (`self.GetActorUpVector`) 0.2)) 100.0) false "None")))
    (`PrimitiveComponent.SetPhysicsAngularVelocityInDegrees` (`self.VisualStaticMeshComponent`) (`KismetMathLibrary.MakeVector` (`KismetMathLibrary.RandomFloatInRange` -500.0 500.0) (`KismetMathLibrary.RandomFloatInRange` -500.0 500.0) (`KismetMathLibrary.RandomFloatInRange` -500.0 500.0)) false "None")))

(fn `IsDamageable`
  (params (TeamID :type String))
  (returns (Return :type Boolean))
  (return false))

(fn `OnRep_Grabber`
  (`/Engine/EditorBlueprintResources/ActorMacros.Switch Has Authority`
    (:`Remote`
      (bind (_success _reference) (message `/Game/RPGSystem/Blueprints/Utilities/BPI_RPG_PlayerCharacter.GetRPGSystem` (`GameplayStatics.GetPlayerCharacter` 0)))
      (if _success
        (set `self.Client_Grabbed` (`KismetArrayLibrary.Array_Contains` (`self.Grabber`) (`/Game/RPGSystem/Blueprints/BPC_RPGSystem.UniqueID` _reference)))
        (`self.SetActorEnableCollision` false)
        (`self.SelectInteractable` false)
        (`self.SetActorHiddenInGame` true)))))

(fn `OnRep_Item`
  (`self.OnItemInfoUpdated`)
  (bind _iteminfo (`self.InitItemInfo`))
  (`self.SetupAppearance` _iteminfo))

(fn `OnRep_Transform`
  (if (not (`KismetMathLibrary.NearlyEqual_TransformTransform` (`self.GetTransform`) (`self.Transform`) 0.01 0.1))
    (`self.SetActorTickEnabled` true)))

(fn `PlayItemTypeDropSound`
  (locals (VarSound :type "SoundBase Object Reference")))

(fn `PlayRarityDropSound`
  (locals (VarSound :type "SoundBase Object Reference"))
  (bind _output_get (set `local.VarSound` (`BlueprintMapLibrary.Map_Find` (`self.RarityDropSound`) (`.Rarity_78_C81B885D4BCDFA0088309599CDCB283C` (break `/Game/RPGSystem/Blueprints/Structure/Inventory/S_Inventory` (`self.Item`))))))
  (`/Engine/EditorBlueprintResources/StandardMacros.IsValid` _output_get
    (:`Is Valid`
      (`GameplayStatics.SpawnSoundAttached` (`local.VarSound`) (`self.DefaultSceneRoot`) "None" (0.0 0.0 0.0) (struct) "SnapToTarget" false 1.0 1.0 0.0 "/Game/RPGSystem/Sound/Attenuation/SA_ItemDrop_Rarity.SA_ItemDrop_Rarity" "/Game/RPGSystem/Sound/Attenuation/ItemDrop_Rarity_Concurrency.ItemDrop_Rarity_Concurrency"))))

(fn `SetParticleColor`
  (params (Color :type "LinearColor Structure"))
  (`FXSystemComponent.SetColorParameter` (`self.RarityParticle`) "Color" Color))

(fn `SetupAppearance`
  (params (ItemInfo :type "/Game/RPGSystem/Blueprints/Structure/Item/S_Item Structure (by ref)"))
  (bind ((`EquipmentSetID_492_F3CF6A5F4135E759D1E70E9AC03925E2` _equipmentsetid) (`BlueprintSettings_465_835AD89D44481B6D40315E9B17E116F0` _blueprintsettings)) (break `/Game/RPGSystem/Blueprints/Structure/Item/S_Item` ItemInfo))
  (bind ((`ItemID_73_6C4D3C2D4D49AA75490544AC57C7939B` _itemid) (`Rarity_78_C81B885D4BCDFA0088309599CDCB283C` _rarity)) (break `/Game/RPGSystem/Blueprints/Structure/Inventory/S_Inventory` (`self.Item`)))
  (bind (_staticmesh _skeletalmesh _meshoffset) (break `/Game/RPGSystem/Blueprints/Structure/Item/S_Item_BlueprintDrop_Settings` _blueprintsettings))
  (if (`self.bDisableVisualSetup`)
    _
    (elif (!= (`self.LastItemID`) _itemid)
      (set `self.LastItemID` _itemid)
      (if (`KismetSystemLibrary.IsValidSoftObjectReference` _staticmesh)
        (`self.LoadtStaticMeshAsync` _staticmesh _meshoffset)
        (`self.SetParticleColor` (`/Game/RPGSystem/Blueprints/Utilities/BPL_RPG_Utilities.Get Rarity Color` _rarity (!= _equipmentsetid "None")))
        (else
          (`self.CheckEnablePhysic`))))))

(fn `UserConstructionScript`
  (if (`self.Persistant`)
    (if (not (`self.bDisableVisualSetup`))
      (bind _returnvalue (`|GetDataTableRow` (`self.Item_DT`) (`.ItemID_73_6C4D3C2D4D49AA75490544AC57C7939B` (break `/Game/RPGSystem/Blueprints/Structure/Inventory/S_Inventory` (`self.Item`))))
        (:`then`
          (bind (_staticmesh _skeletalmesh _meshoffset) (break `/Game/RPGSystem/Blueprints/Structure/Item/S_Item_BlueprintDrop_Settings` (`.BlueprintSettings_465_835AD89D44481B6D40315E9B17E116F0` (break `/Game/RPGSystem/Blueprints/Structure/Item/S_Item` _returnvalue))))
          (if (`KismetSystemLibrary.IsValidSoftObjectReference` _staticmesh)
            (`KismetSystemLibrary.LoadAsset_Blocking` _staticmesh)
            (`self.InitVisualMesh` (`|ConvertAsset` _staticmesh) _meshoffset)
            (`self.OnAsyncLoadStaticMeshFinished`)))))))