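; Player camera manager for the RPG system, adding HUD-layer screen fades, top-down spring arm zoom and camera velocity tracking.
; Fade events drive a WBP_CustomFade widget updated on Tick, using a transparent native camera fade only to fade audio.
; Tick also eases a clamped zoom value that blends spring arm length and pitch, and records the frame-to-frame camera position delta as velocity.
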(event `self.ReceiveBeginPlay`)

(event `/Game/RPGSystem/Blueprints/Utilities/BPI_RPG_PlayerCamera.SetManualCameraFadeWithHUD`
  (params (FadeAmount :type "Float (double-precision)") (Color :type "LinearColor Structure") (FadeAudio :type Boolean))
  (bind _customfadewidget (`self.CustomFadeWidget`))
  (bind _customfadewidget_2 (`self.CustomFadeWidget`))
  ;[1 1 1] Set Fade
  (if (== FadeAmount 0.0)
    (`/Engine/EditorBlueprintResources/StandardMacros.IsValid` _customfadewidget_2
      (:`Is Valid`
        (`Widget.RemoveFromParent` _customfadewidget_2)
        (set `self.CustomFadeWidget` null)
        (set `self.Hold when Finished` false)))
    (else
      (set `self.Hold when Finished` true)
      (`/Engine/EditorBlueprintResources/StandardMacros.IsValid` (`self.CustomFadeWidget`)
        (:`Is Valid`
          (`/Game/RPGSystem/Blueprints/UI/WBP_CustomFade.UpdateColor` _customfadewidget Color)
          (`/Game/RPGSystem/Blueprints/UI/WBP_CustomFade.UpdateFade` _customfadewidget FadeAmount))
        (:`Is Not Valid`
          (bind _returnvalue (`|CreateWidget` "/Game/RPGSystem/Blueprints/UI/WBP_CustomFade.WBP_CustomFade_C" null Color FadeAmount))
          (bind _output_get (set `self.CustomFadeWidget` _returnvalue))
          (`UserWidget.AddToViewport` _output_get (`self.CustomFade_ZOrder`))))
      (if FadeAudio
        (`self.SetManualCameraFade` FadeAmount (struct) true)))))

(event `/Game/RPGSystem/Blueprints/Utilities/BPI_RPG_PlayerCamera.StartCameraFadeWithHUD`
  (params (FromAlpha :type "Float (double-precision)") (ToAlpha :type "Float (double-precision)") (Duration :type "Float (double-precision)") (Color :type "LinearColor Structure") (FadeAudio :type Boolean) (HoldWhenFinished :type Boolean))
  (bind _customfadewidget (`self.CustomFadeWidget`))
  (`/Engine/EditorBlueprintResources/StandardMacros.IsValid` (`self.CustomFadeWidget`)
    (:`Is Valid`
      (`/Game/RPGSystem/Blueprints/UI/WBP_CustomFade.UpdateColor` _customfadewidget Color)
      (`/Game/RPGSystem/Blueprints/UI/WBP_CustomFade.UpdateFade` _customfadewidget FromAlpha))
    (:`Is Not Valid`
      (bind _returnvalue (`|CreateWidget` "/Game/RPGSystem/Blueprints/UI/WBP_CustomFade.WBP_CustomFade_C" null Color FromAlpha))
      (bind _output_get (set `self.CustomFadeWidget` _returnvalue))
      (`UserWidget.AddToViewport` _output_get (`self.CustomFade_ZOrder`))))
  (set `self.FadeFrom` FromAlpha)
  (set `self.FadeDuration` Duration)
  (set `self.FadeToGoal` ToAlpha)
  (set `self.StartFadeFinishTime` (+ (`self.GetGameTimeSinceCreation`) Duration))
  (set `self.Hold when Finished` HoldWhenFinished)
  (set `self.FadingWithHUD` true)
  (`self.SetActorTickEnabled` true)
  (if FadeAudio
    (`self.StartCameraFade` (`self.FadeFrom`) (`self.FadeToGoal`) (`self.FadeDuration`) (struct) true (`self.Hold when Finished`))))

(event `/Game/RPGSystem/Blueprints/Utilities/BPI_RPG_PlayerCamera.StopCameraFadeWithHUD`
  (bind _customfadewidget (`self.CustomFadeWidget`))
  (`/Engine/EditorBlueprintResources/StandardMacros.IsValid` _customfadewidget
    (:`Is Valid`
      (`Widget.RemoveFromParent` _customfadewidget)
      (set `self.CustomFadeWidget` null))
    (:`Is Not Valid`
      _))
  (`self.SetActorTickEnabled` false)
  (set `self.FadingWithHUD` false)
  (`self.StopCameraFade`))

(event `/Game/RPGSystem/Blueprints/Utilities/BPI_RPG_PlayerCamera.SetSpringArm_TopDown`
  (params (SpringArm :type "SpringArmComponent Object Reference") (Length_Zoomed :type "Float (double-precision)"))
  ;[1 1 1] Comment
  (set `self.SpringArmLengthZoomed` 600.0)
  (set `self.CameraDefaultRotation` (`SceneComponent.RelativeRotation` SpringArm))
  (set `self.SpringArmLengthDefault` (`SpringArmComponent.TargetArmLength` SpringArm))
  (set `self.SpringArm` SpringArm))

(event `/Game/RPGSystem/Blueprints/Utilities/BPI_RPG_PlayerCamera.SetCameraZoomValue`
  (params (Value :type "Float (double-precision)"))
  ;[1 1 1] Camera Zoom Value
  (set `self.CameraZoomValueGoal` (`KismetMathLibrary.FClamp` Value)))

(event `self.ReceiveTick`
  (params (DeltaSeconds :type "Float (single-precision)"))
  (bind _customfadewidget (`self.CustomFadeWidget`))
  (bind _returnvalue (- (`self.StartFadeFinishTime`) (`self.GetGameTimeSinceCreation`)))
  (`self.HandleCameraZoomAndRotation_TopDown` DeltaSeconds) ; Move to child
  ;[1 1 1] Camera Velocity
  (set `self.CameraVelocity` (- (`self.LastCameraPosition`) (`self.GetCameraLocation`)))
  (set `self.LastCameraPosition` (`self.GetCameraLocation`))
  ;[1 1 1] Custom Fade Tick
  (if (`self.FadingWithHUD`)
    (`/Game/RPGSystem/Blueprints/UI/WBP_CustomFade.UpdateFade` (`self.CustomFadeWidget`) (`KismetMathLibrary.MapRangeClamped` _returnvalue (`self.FadeDuration`) 0.0 (`self.FadeFrom`) (`self.FadeToGoal`)))
    (if (and (or (not (`self.Hold when Finished`)) (<= (`self.FadeToGoal`) 0.0)) (< _returnvalue 0.0))
      (set `self.FadingWithHUD` false))
    (else
      (`/Engine/EditorBlueprintResources/StandardMacros.IsValid` _customfadewidget
        (:`Is Valid`
          (`Widget.RemoveFromParent` _customfadewidget)
          (set `self.CustomFadeWidget` null))))))

(event `/Game/RPGSystem/Blueprints/Utilities/BPI_RPG_PlayerCamera.AddCameraRotationValue`
  (params (Value :type "Float (double-precision)"))
  ;[1 1 1] Camera Zoom Value
  (set `self.CameraZoomValueGoal` (`KismetMathLibrary.FClamp` (+ Value (`self.CameraZoomValueGoal`)))))

(fn `GetCameraVelocity`
  (returns (Return :type "Vector Structure"))
  (return (`self.CameraVelocity`)))

(fn `HandleCameraZoomAndRotation_TopDown`
  (params (Delta :type "Float (double-precision)"))
  (bind _springarm (`self.SpringArm`))
  (bind _springarm_2 (`self.SpringArm`))
  (bind _roll (.roll (`SceneComponent.RelativeRotation` _springarm)))
  (bind _yaw (.yaw (`SceneComponent.RelativeRotation` _springarm)))
  (`/Engine/EditorBlueprintResources/StandardMacros.IsValid` _springarm
    (:`Is Valid`
      (set `self.CameraZoomValue` (`KismetMathLibrary.Lerp` (`self.CameraZoomValue`) (`self.CameraZoomValueGoal`) (* Delta (`self.CameraZoomLerpStrength`))))
      (`SceneComponent.K2_SetRelativeRotation` _springarm_2 (`KismetMathLibrary.RLerp` (`KismetMathLibrary.MakeRotator` _roll (.pitch (`self.CameraDefaultRotation`)) _yaw) (`KismetMathLibrary.MakeRotator` _roll -10.0 _yaw) (`self.CameraZoomValue`) true) false true)
      (set `SpringArmComponent.TargetArmLength` (`KismetMathLibrary.Lerp` (`self.SpringArmLengthDefault`) (`self.SpringArmLengthZoomed`) (`self.CameraZoomValue`)) _springarm_2))))

(fn `UserConstructionScript`)