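; Camera modifier that applies a blindness post-process effect in the RPG system, leaving view location, rotation and FOV untouched.
; Each update raises BlendInAlpha toward 1 at a rate that slows as it grows, using it as the post-process weight.
; Once fully blended in, the weight switches to the modifier's own Alpha, so it then follows that value.
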(fn `BlueprintModifyCamera`
  (params (DeltaTime :type "Float (single-precision)") (ViewLocation :type "Vector Structure") (ViewRotation :type "Rotator Structure") (FOV :type "Float (single-precision)"))
  (returns (NewViewLocation :type "Vector Structure") (NewViewRotation :type "Rotator Structure") (NewFOV :type "Float (single-precision)"))
  (return ViewLocation ViewRotation FOV))

(fn `BlueprintModifyPostProcess`
  (params (DeltaTime :type "Float (single-precision)"))
  (returns (PostProcessBlendWeight :type "Float (single-precision)") (PostProcessSettings :type "PostProcessSettings Structure"))
  (bind _output_get (set `self.Blend_In_Alpha` (`KismetMathLibrary.FMin` (+ (stale _output_get) (* DeltaTime (+ (* (- 1.0 (`KismetMathLibrary.SafeDivide` (`self.Blend_In_Alpha`) 3.0)) 3.0) 0.01))) 1.0)))
  (return (`KismetMathLibrary.SelectFloat` (`self.Alpha`) _output_get (>= _output_get 1.0)) (make `PostProcessSettings` :`VignetteIntensity` 3.0)))